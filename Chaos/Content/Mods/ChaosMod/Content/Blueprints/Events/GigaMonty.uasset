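; Chaos Mod event actor that spawns a MontyShowtimeMission AI running MontyShowtimeBT and brings it back whenever it is gone.
; BeginPlay spawns it at the event actor's position, then sets the Giga flag after a short delay so later spawns use the saved location.
; Tick records the AI's position about once a second and uses a DoOnce, re-armed while the AI is valid, to respawn it there.
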(event EventBeginPlay
  (bind _returnvalue (AI|SpawnAIFromClass "/Game/Blueprints/AI/Seeker/Monty/MontyShowtime/MontyShowtimeMission.MontyShowtimeMission_C" "/Game/Blueprints/AI/Seeker/Monty/MontyShowtime/MontyShowtimeBT.MontyShowtimeBT" (select (Variables|Default|GetGiga) (Variables|Default|GetLocation) (Transformation|GetActorLocation)) "0, 0, 0" false 0))
  (Utilities|FlowControl|Delay 1.0)
  (Variables|Default|SetGiga true))

(event EventTick
  (params (DeltaSeconds :type Float%20%28single-precision%29))
  (Utilities|FlowControl|Sequence
    (:then_0
      (Utilities|IsValid (stale _returnvalue)
        (:Is%20Valid
          (goto _label Reset))
        (:Is%20Not%20Valid
          (Utilities|FlowControl|DoOnce true :!label _label
            (:Completed
              (bind _returnvalue (AI|SpawnAIFromClass "/Game/Blueprints/AI/Seeker/Monty/MontyShowtime/MontyShowtimeMission.MontyShowtimeMission_C" "/Game/Blueprints/AI/Seeker/Monty/MontyShowtime/MontyShowtimeBT.MontyShowtimeBT" (select (Variables|Default|GetGiga) (Variables|Default|GetLocation) (Transformation|GetActorLocation)) "0, 0, 0" false 0))
              (Utilities|FlowControl|Delay 1.0)
              (Variables|Default|SetGiga true))))))
    (:then_1
      (Utilities|FlowControl|Delay 1.0)
      (Variables|Default|SetLocation (Transformation|GetActorLocation _returnvalue)))))

(fn ConstructionScript)