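; ButtonActor is a ChaosMod actor that wraps a toggle button and raises an OnButtonPressed event when it is switched on.
; On BeginPlay it spawns a BasicToggleButton at its own transform and keeps a reference to it.
; Tick polls the button's state and uses a DoOnce to fire the event once per press.
; With AutoReset set, it waits ResetTime, then clears the button and re-arms; Reset does the same.
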(event Custom|Reset
  (Variables|/Game/Blueprints/Button/BasicToggleButton.BasicToggleButton_C|SetState (Variables|Default|GetButton) false)
  (Utilities|FlowControl|DoOnce false) ; enters at Reset
)

(event EventBeginPlay
  (bind _returnvalue (Game|SpawnActorfromClass "/Game/Blueprints/Button/BasicToggleButton.BasicToggleButton_C" (Transformation|GetActorTransform) "Undefined" 0 0))
  (Variables|Default|SetButton _returnvalue))

(event EventTick
  (params (DeltaSeconds :type Float%20%28single-precision%29))
  (if (Variables|/Game/Blueprints/Button/BasicToggleButton.BasicToggleButton_C|GetState (Variables|Default|GetButton))
    (Utilities|FlowControl|DoOnce false
      (:Completed
        (Default|CallOnButtonPressed)
        (if (Variables|Default|GetAutoReset)
          (Utilities|FlowControl|Delay (Variables|Default|GetResetTime))
          (CallFunction|Reset))))))

(fn ConstructionScript)