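; Chaos mod event actor "Heavy" that applies an animated full-screen post-process effect.
; On BeginPlay it finds the ModActor, creates a dynamic instance of PP_Heavy and appends it at full weight to that actor's PostProcess materials.
; Tick advances a time-scaled counter and writes it to the material's "x" scalar parameter to drive the animation.
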(event EventTick
  (params (DeltaSeconds :type Float%20%28single-precision%29))
  (bind _output_get (Variables|Default|Setx (+ (Variables|Default|Getx) (* 3 DeltaSeconds))))
  (Rendering|Material|SetScalarParameterValue (stale EventBeginPlay _returnvalue_2) "x" _output_get :!class /Script/Engine.MaterialInstanceDynamic))

(event EventBeginPlay
  (bind _returnvalue (Actor|GetActorOfClass "/Game/Mods/ChaosMod/ModActor.ModActor_C"))
  (Variables|Default|SetModActor _returnvalue)
  (bind _returnvalue_2 (Rendering|Material|CreateDynamicMaterialInstance "/Game/Mods/ChaosMod/Content/Materials/PP_Heavy.PP_Heavy" "None" "None" :!class /Script/Engine.KismetMaterialLibrary))
  (Utilities|Array|AppendArray (.array (Utilities|Struct|BreakPostProcessSettings (Variables|/Script/Engine.PostProcessComponent|GetSettings (Variables|/Game/Mods/ChaosMod/ModActor.ModActor_C|GetPostProcess (Variables|Default|GetModActor))))) (Utilities|Array|MakeArray (Utilities|Struct|MakeWeightedBlendable 1.0 _returnvalue_2))))

(fn ConstructionScript)