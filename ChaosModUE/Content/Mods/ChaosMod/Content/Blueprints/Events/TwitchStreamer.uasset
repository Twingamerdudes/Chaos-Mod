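; Chaos mod Twitch Streamer event that puts a Streamer widget on screen, using the player's webcam when one works.
; On BeginPlay it enumerates video capture devices and tries each URL on the media player through a callback-driven blocking loop that advances on failure.
; An opened device gets a video track selected and played before the webcam widget appears.
; Without a working device, a delayed fallback creates the widget without webcam.
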(event Custom|OnMediaOpened
  (params (OpenedUrl :type String))
  (bind _mp (Variables|Default|GetMP))
  (bind _index (Utilities|FlowControl|ForLoopwithBreak 0 (- (Class|MediaPlayer|GetNumTracks _mp "Video") 1) :!label _label)
    (:LoopBody
      (if (> (Class|MediaPlayer|GetNumTrackFormats _mp "Video" _index) 0)
        (bind _returnvalue (Class|MediaPlayer|SelectTrack _mp "Video" _index))
        (if _returnvalue
          (Utilities|FlowControl|Delay 2.0)
          (bind _returnvalue_2 (Media|MediaPlayer|Play _mp :!class /Script/MediaAssets.MediaPlayer))
          (if _returnvalue_2
            (bind _returnvalue_3 (UserInterface|CreateWidget "/Game/Mods/ChaosMod/Content/Blueprints/Widgets/Events/Streamer.Streamer_C" 0 true))
            (UserInterface|Viewport|AddtoViewport _returnvalue_3 0)
            (Variables|Default|SetGood true)
            (goto _label Break)))))
    (:Completed
      (Utilities|FlowControl|Delay 4.0)
      (if (not (Variables|Default|GetGood))
        (bind _returnvalue_4 (UserInterface|CreateWidget "/Game/Mods/ChaosMod/Content/Blueprints/Widgets/Events/Streamer.Streamer_C"))
        (UserInterface|Viewport|AddtoViewport _returnvalue_4 0)))))

(event Custom|OnMediaOpenFailed
  (params (FailedUrl :type String))
  (Utilities|CustomforEachLoopBlocking (stale EventBeginPlay _outdevices)) ; enters at CallbackReady
)

(event EventBeginPlay
  (bind _mp (Variables|Default|GetMP))
  (EventDispatchers|AssignOnMediaOpened _mp (delegate Custom|OnMediaOpened))
  (EventDispatchers|AssignOnMediaOpenFailed _mp (delegate Custom|OnMediaOpenFailed))
  (bind _outdevices (Class|MediaBlueprintFunctionLibrary|EnumerateVideoCaptureDevices (|BitmaskLiteral 15)))
  (if (>= (Utilities|Array|Length _outdevices) 1)
    (bind _element (Utilities|CustomforEachLoopBlocking _outdevices :!label _label)
      (:Loop%20Body
        (bind _returnvalue (Class|MediaPlayer|OpenUrl (Variables|Default|GetMP) (.url _element)))
        (if (not _returnvalue)
          (goto _label CallbackReady)))
      (:Completed
        (Utilities|FlowControl|Delay 4.0 :!label _label_2)
        (if (not (Variables|Default|GetGood))
          (bind _returnvalue_2 (UserInterface|CreateWidget "/Game/Mods/ChaosMod/Content/Blueprints/Widgets/Events/Streamer.Streamer_C"))
          (UserInterface|Viewport|AddtoViewport _returnvalue_2 0))))
    (else
      (goto _label_2))))

(fn ConstructionScript)