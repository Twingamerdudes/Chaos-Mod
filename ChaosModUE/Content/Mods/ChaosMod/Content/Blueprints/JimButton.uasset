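; JimButton is a ChaosMod novelty button actor that plays a "Jim" sound when activated.
; On BeginPlay it spawns a BasicToggleButton at its own transform and polls that button's State on Tick.
; A DoOnce gates each press, firing an attached, attenuated sound and a timeline that drives the skeletal mesh's "Push" morph target.
; A short delay then clears the state and re-arms the gate, turning the toggle into a momentary button.
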(event Custom|SayJim
  (Audio|SpawnSoundAttached "/Game/Mods/ChaosMod/Content/Audio/JimButton.JimButton" (Variables|Default|GetSkeletalMesh) "None" "0, 0, 0" "0, 0, 0" "KeepRelativeOffset" false 1.0 1.0 0.0 "/Game/Mods/ChaosMod/Content/Audio/JimAtten.JimAtten" 0)
  (bind _newtrack_0 (Timeline|Timeline_0 PlayFromStart)
    (:Update
      (Components|SkeletalMesh|SetMorphTarget (Variables|Default|GetSkeletalMesh) "Push" _newtrack_0 true))))

(event Custom|Reset
  (Variables|/Game/Blueprints/Button/BasicToggleButton.BasicToggleButton_C|SetState (Variables|Default|GetButton) false)
  (Utilities|FlowControl|DoOnce false) ; enters at Reset
)

(event EventBeginPlay
  (bind _returnvalue (Game|SpawnActorfromClass "/Game/Blueprints/Button/BasicToggleButton.BasicToggleButton_C" (Transformation|GetActorTransform) "Undefined" 0 0))
  (Variables|Default|SetButton _returnvalue))

(event Collision|EventActorBeginOverlap
  (params (OtherActor :type Actor%20Object%20Reference)))

(event EventTick
  (params (DeltaSeconds :type Float%20%28single-precision%29))
  (if (Variables|/Game/Blueprints/Button/BasicToggleButton.BasicToggleButton_C|GetState (Variables|Default|GetButton))
    (Utilities|FlowControl|DoOnce false
      (:Completed
        (CallFunction|SayJim)
        (Utilities|FlowControl|Delay 0.6)
        (CallFunction|Reset)))))

(fn ConstructionScript)