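; CubeOfDeath is a chaos mod event actor that kills Gregory when he is caught inside it.
; On BeginPlay it plays the Ascend level sequence.
; Once that sequence stops, Tick checks whether its Sphere overlaps Gregory and, a single time, shows a FLASHBANG widget, waits two seconds, then calls KillGregory on the ModActor.
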(event EventBeginPlay
  (Sequencer|Player|Play (Variables|/Script/ActorSequence.ActorSequenceComponent|GetSequencePlayer (Variables|Default|GetAscend)) :!class /Script/MovieScene.MovieSceneSequencePlayer))

(event EventTick
  (params (DeltaSeconds :type Float%20%28single-precision%29))
  (if (not (Audio|Components|Audio|IsPlaying (Variables|/Script/ActorSequence.ActorSequenceComponent|GetSequencePlayer (Variables|Default|GetAscend))))
    (bind _returnvalue (Actor|GetActorOfClass "/Game/Blueprints/Player/Gregory.Gregory_C"))
    (if (Collision|IsOverlappingActor (Variables|Default|GetSphere) _returnvalue :!class /Script/Engine.PrimitiveComponent)
      (Utilities|FlowControl|DoOnce false
        (:Completed
          (bind _returnvalue_2 (UserInterface|CreateWidget "/Game/Mods/ChaosMod/Content/Widgets/FLASHBANG.FLASHBANG_C"))
          (UserInterface|Viewport|AddtoViewport _returnvalue_2 2147483647)
          (Utilities|FlowControl|Delay 2.0)
          (bind _returnvalue_3 (Actor|GetActorOfClass "/Game/Mods/ChaosMod/ModActor.ModActor_C"))
          (Default|KillGregory _returnvalue_3))))))

(fn ConstructionScript)