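; ItemManager is a Chaos Mod actor that applies the gameplay effects of purchased items.
; It binds to an item-purchase event, flags the ID in an Items array, and runs one-off effects such as spawning a barrier, maxing stamina or laser shots, attaching a FazGlock to the camera, saving, or disabling jumpscares.
; Tick uses those flags for persistent effects: slowing all AI through time dilation and recharging the Flashbeacon.
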(event Custom|OnItemPurchased_Event
  (params (ID :type Integer))
  (bind _returnvalue (Game|GetPlayerCharacter 0))
  (bind _returnvalue_2 (Subsystems|GetFNAFSaveGameSystem))
  (Utilities|Array|SetArrayElem (Variables|Default|GetItems) ID true)
  (switch int ID
    (:0
      (Game|SpawnActorfromClass "/Game/Mods/ChaosMod/Content/Blueprints/Events/Barrier.Barrier_C" (Math|Transform|MakeTransform "0, 0, 0" "0, 0, 0" "1,1,1") "Undefined" 0 0))
    (:1
      (Variables|/Game/Blueprints/Player/StaminaComponent.StaminaComponent_C|SetCurrentStamina (Actor|GetComponentbyClass (Game|Player|GetPlayerPawn 0) "/Game/Blueprints/Player/StaminaComponent.StaminaComponent_C") 999999986991104.0))
    (:3
      (bind _returnvalue_3 (Actor|GetActorOfClass "/Game/Blueprints/Objects/Equippables/EQ_LaserGun.EQ_LaserGun_C"))
      (Variables|/Game/Blueprints/Objects/Equippables/EQ_LaserGun.EQ_LaserGun_C|SetShotsLeft _returnvalue_3 10000000))
    (:4
      (bind _asgregory (Utilities|Casting|CastToGregory _returnvalue))
      (Default|SwitchItemwithAnim _asgregory)
      (Utilities|FlowControl|Delay 0.4)
      (bind _returnvalue_4 (Game|AddComponentbyClass _returnvalue "/Script/Engine.ChildActorComponent" false))
      (Transformation|AttachComponentToComponent _returnvalue_4 (Actor|GetComponentbyClass _returnvalue "/Script/Engine.CameraComponent") "None" "SnapToTarget" "SnapToTarget" "SnapToTarget" true)
      (ChildActorComponent|SetChildActorClass _returnvalue_4 "/Game/Mods/ChaosMod/Content/Blueprints/FazGlock.FazGlock_C"))
    (:6
      (Class|FNAFSaveGameSystem|AsyncSaveGame _returnvalue_2 (Variables|/Script/fnaf9.FNAFSaveGameSystem|GetSaveSlotName _returnvalue_2) false false))
    (:7
      (bind _returnvalue_5 (Actor|GetActorOfClass "/Game/Blueprints/Player/Gregory.Gregory_C"))
      (Variables|/Game/Blueprints/Player/Gregory.Gregory_C|SetCanBeJumpScared _returnvalue_5 false))))

(event EventBeginPlay
  (bind _returnvalue (Actor|GetActorOfClass "/Game/Mods/ChaosMod/ModActor.ModActor_C"))
  (Variables|Default|SetModActor _returnvalue)
  (EventDispatchers|BindEventtoOnItemPurchased (delegate Custom|OnItemPurchased_Event)))

(event EventTick
  (params (DeltaSeconds :type Float%20%28single-precision%29))
  (bind _items (Variables|Default|GetItems))
  (Utilities|FlowControl|Sequence
    (:then_0
      (if (Utilities|Array|Get(acopy) _items 2)
        (for _array_element (Class|AIManagementSystem|GetAllAI (Subsystems|GetAIManagementSystem))
          (Variables|/Script/Engine.Actor|SetCustomTimeDilation _array_element 0.5))))
    (:then_1
      (if (Utilities|Array|Get(acopy) _items 3)
        (bind _returnvalue (Actor|GetActorOfClass "/Game/Blueprints/Objects/Equippables/EQ_Flashbeacon.EQ_Flashbeacon_C"))
        (if (not (Variables|/Game/Blueprints/Objects/Equippables/EQ_Flashbeacon.EQ_Flashbeacon_C|GetCanUse? _returnvalue))
          (Utilities|DoOnce(selfReset) false 1.2)
          (Default|Recharging _returnvalue))))))

(fn ConstructionScript)