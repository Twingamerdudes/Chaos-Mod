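; Turret actor for ChaosMod that automatically stuns nearby AI seekers it has line of sight to.
; Each Tick while off cooldown, it scans all AISeeker actors within StunRadius and confirms each with a complex Visibility trace before calling Stun.
; A hit starts a Delay-based cooldown, but the loop does not break, so every visible seeker in range is stunned in the same pass.
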(event Custom|CoolDown
  (Variables|Default|SetCoolingDown true)
  (Utilities|FlowControl|Delay (Variables|Default|GetCoolDownTime))
  (Variables|Default|SetCoolingDown false))

(event EventBeginPlay)

(event Collision|EventActorBeginOverlap
  (params (OtherActor :type Actor%20Object%20Reference)))

(event EventTick
  (params (DeltaSeconds :type Float%20%28single-precision%29))
  (bind _self self)
  (if (not (Variables|Default|GetCoolingDown))
    (bind _outactors (Actor|GetAllActorsOfClass "/Game/Blueprints/AI/Seeker/AISeeker.AISeeker_C"))
    (for _array_element _outactors
      (if (< (Transformation|GetDistanceTo _array_element _self) (Variables|Default|GetStunRadius))
        (bind _outhit (Collision|LineTraceByChannel (Transformation|GetActorLocation _self) (Transformation|GetActorLocation _array_element) "TraceTypeQuery1" true 0 "None"))
        (if (== (.HitActor (Collision|BreakHitResult _outhit)) _array_element)
          (Default|Stun _array_element)
          (CallFunction|CoolDown))))))

(fn ConstructionScript)