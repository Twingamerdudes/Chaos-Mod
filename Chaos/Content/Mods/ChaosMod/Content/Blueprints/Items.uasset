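; Chaos mod actor that applies the effects of item perks flagged in an Items array.
; On Tick, one flag repeatedly sets half time dilation on a hardcoded list of enemy classes through a delayed EnemyDilation call.
; Another auto-recharges the Fazerblaster and Fazcam found at BeginPlay, throttling the camera with a DoOnce and delay.
; A further flag lets the G key toggle a Gun actor by spawning or destroying it.
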(event EventTick
  (params (DeltaSeconds :type Float%20%28single-precision%29))
  (bind _items (Variables|Default|GetItems))
  (bind _fazcam (Variables|Default|GetFazcam))
  (bind _fazerblaster (Variables|Default|GetFazerblaster))
  (Utilities|FlowControl|Sequence
    (:then_0
      (if (Utilities|Array|Get(acopy) _items 2)
        (Utilities|FlowControl|Delay 2.0)
        (Utilities|EnemyDilation 0.5)))
    (:then_1
      (if (Utilities|Array|Get(acopy) _items 3)
        (Utilities|FlowControl|Sequence
          (:then_0
            (if (<= (Variables|/Game/Blueprints/Objects/Equippables/EQ_LaserGun.EQ_LaserGun_C|GetShotsLeft _fazerblaster) 5)
              (Default|Recharge _fazerblaster)))
          (:then_1
            (if (not (Variables|/Game/Blueprints/Objects/Equippables/EQ_Flashbeacon.EQ_Flashbeacon_C|GetCanUse? _fazcam))
              (Utilities|FlowControl|DoOnce false :!label _label
                (:Completed
                  (Default|Recharging _fazcam)
                  (Utilities|FlowControl|Delay 1.2)
                  (goto _label Reset))))))))))

(event EventBeginPlay
  (bind _returnvalue (Actor|GetActorOfClass "/Game/Blueprints/Objects/Equippables/EQ_Flashbeacon.EQ_Flashbeacon_C"))
  (Variables|Default|SetFazcam _returnvalue)
  (bind _returnvalue_2 (Actor|GetActorOfClass "/Game/Blueprints/Objects/Equippables/EQ_LaserGun.EQ_LaserGun_C"))
  (Variables|Default|SetFazerblaster _returnvalue_2))

(event Input|KeyboardEvents|G
  (params (Key :type Key%20Structure :default "None"))
  (:Pressed
    (if (Utilities|Array|Get(acopy) (Variables|Default|GetItems) 4)
      (if (Variables|Default|GetGun%20Stored)
        (Variables|Default|SetGun%20Stored false)
        (Game|SpawnActorfromClass "/Game/Mods/ChaosMod/Content/Blueprints/Events/Gun.Gun_C" (Math|Conversions|ToTransform(Vector) "0, 0, 0") "Undefined" 0 0)
        (else
          (Variables|Default|SetGun%20Stored true)
          (bind _returnvalue (Actor|GetActorOfClass "/Game/Mods/ChaosMod/Content/Blueprints/Events/Gun.Gun_C"))
          (Actor|DestroyActor _returnvalue))))))

(fn ConstructionScript)