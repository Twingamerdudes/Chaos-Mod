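; Chaos Mod event actor that rewinds the player's movement, then destroys itself.
; While the Record flag is set, Tick stores the pawn's location and control rotation every frame.
; Ten seconds after BeginPlay, recording stops, move and look input are ignored, and a delay-driven reverse loop steps back through the samples, teleporting the pawn and restoring view rotation.
; Input is restored when the rewind ends.
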(event EventTick
  (params (DeltaSeconds :type Float%20%28single-precision%29))
  (if (Variables|Default|GetRecord)
    (Utilities|Array|Add (Variables|Default|GetTransform) (Math|Transform|MakeTransform (Transformation|GetActorLocation (Game|Player|GetPlayerPawn 0)) (Pawn|GetControlRotation (Game|GetPlayerController 0) :!class /Script/Engine.Controller) "1,1.000000,1"))))

(event EventBeginPlay
  (bind _returnvalue (Game|GetPlayerController 0))
  (bind _returnvalue_2 (Game|GetPlayerController 0))
  (bind _variable (|TemporaryVariable))
  (bind _variable_2 (|TemporaryVariable))
  (bind _transform (Variables|Default|GetTransform))
  (bind _returnvalue_3 (Utilities|Array|Length _transform))
  (bind _output (Utilities|Array|Get(acopy) _transform _variable))
  (bind _returnvalue_4 (- _returnvalue_3 1))
  (Utilities|FlowControl|Delay 1e+01)
  (Variables|Default|SetRecord false)
  (Input|SetIgnoreMoveInput _returnvalue_2 true)
  (Input|SetIgnoreLookInput _returnvalue_2 true)
  (|Assign _variable_2 _returnvalue_4)
  (|Assign _variable (Math|Integer|Max(Integer) 0 _returnvalue_4))
  (if (>= _variable_2 0) :!label _label
    (|Assign _variable _variable_2)
    (Utilities|FlowControl|Delay (Utilities|Time|GetWorldDeltaSeconds))
    (Utilities|FlowControl|Sequence
      (:then_0
        (Transformation|SetActorLocation (Game|Player|GetPlayerPawn 0) (.location _output) false false)
        (Pawn|SetControlRotation (Game|GetPlayerController 0) (.rotation _output)))
      (:then_1
        (|Assign _variable_2 (- _variable_2 1))
        (goto _label)))
    (else
      (Input|SetIgnoreMoveInput _returnvalue false)
      (Input|SetIgnoreLookInput _returnvalue false)
      (Actor|DestroyActor))))

(fn ConstructionScript)