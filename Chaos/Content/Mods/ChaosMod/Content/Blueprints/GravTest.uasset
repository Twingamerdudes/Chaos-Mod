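; GravTest is a ChaosMod test Blueprint that toggles a random custom gravity on physics objects and characters.
; It attaches GravityComponents to physics-simulating actors and all Characters, storing them in an array, at BeginPlay in unpackaged builds and two seconds after every level update.
; Only the non-Character pass skips actors that already have one.
; Its gravityevent alternates between applying one shared random gravity vector and switching custom gravity off.
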(event Custom|OnlevelsUpdated_Event_0
  (Utilities|FlowControl|Delay 2.0)
  (bind _outactors (Actor|GetAllActorsOfClass "/Script/Engine.Actor"))
  (for _array_element _outactors
    (if (not (> (Utilities|Array|Length (Actor|GetComponentsByClass _array_element "/Game/Mods/ChaosMod/Content/Blueprints/Events/GravityComponent.GravityComponent_C")) 0))
      (bind _array_element_2 (Utilities|Array|ForEachLoopwithBreak (Actor|GetComponentsByClass _array_element "/Script/Engine.PrimitiveComponent") :!label _label)
        (:LoopBody
          (if (and (Physics|IsSimulatingPhysics _array_element_2 "None") (Class|PrimitiveComponent|IsGravityEnabled _array_element_2))
            (bind _returnvalue (Game|AddComponentbyClass _array_element "/Game/Mods/ChaosMod/Content/Blueprints/Events/GravityComponent.GravityComponent_C"))
            (Utilities|Array|Add (Variables|Default|GetST) _returnvalue)
            (goto _label Break))))))
  (bind _outactors_2 (Actor|GetAllActorsOfClass "/Script/Engine.Character"))
  (for _array_element_3 _outactors_2
    (bind _returnvalue_2 (Game|AddComponentbyClass _array_element_3 "/Game/Mods/ChaosMod/Content/Blueprints/Events/GravityComponent.GravityComponent_C"))
    (Utilities|Array|Add (Variables|Default|GetST) _returnvalue_2)))

(event Custom|gravityevent
  (Utilities|FlowControl|FlipFlop
    (:A
      (Variables|Default|SetDir (* (Math|Random|RandomUnitVector) 5555))
      (for _array_element (Variables|Default|GetST)
        (Default|SetCustomGravity _array_element true (Variables|Default|GetDir))))
    (:B
      (for _array_element_2 (Variables|Default|GetST)
        (Default|SetCustomGravity _array_element_2 false "0, 0, 0")))))

(event EventBeginPlay
  (EventDispatchers|AssignOnlevelsUpdated (Subsystems|GetFNAFLevelManager) (delegate Custom|OnlevelsUpdated_Event_0))
  (if (not (Class|KismetSystemLibrary|IsPackagedforDistribution))
    (bind _outactors (Actor|GetAllActorsOfClass "/Script/Engine.Actor"))
    (for _array_element _outactors
      (if (not (> (Utilities|Array|Length (Actor|GetComponentsByClass _array_element "/Game/Mods/ChaosMod/Content/Blueprints/Events/GravityComponent.GravityComponent_C")) 0))
        (bind _array_element_2 (Utilities|Array|ForEachLoopwithBreak (Actor|GetComponentsByClass _array_element "/Script/Engine.PrimitiveComponent") :!label _label)
          (:LoopBody
            (if (and (Physics|IsSimulatingPhysics _array_element_2 "None") (Class|PrimitiveComponent|IsGravityEnabled _array_element_2))
              (bind _returnvalue (Game|AddComponentbyClass _array_element "/Game/Mods/ChaosMod/Content/Blueprints/Events/GravityComponent.GravityComponent_C"))
              (Utilities|Array|Add (Variables|Default|GetST) _returnvalue)
              (goto _label Break))))))
    (bind _outactors_2 (Actor|GetAllActorsOfClass "/Script/Engine.Character"))
    (for _array_element_3 _outactors_2
      (bind _returnvalue_2 (Game|AddComponentbyClass _array_element_3 "/Game/Mods/ChaosMod/Content/Blueprints/Events/GravityComponent.GravityComponent_C"))
      (Utilities|Array|Add (Variables|Default|GetST) _returnvalue_2))))

(fn ConstructionScript)