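; Chaos Mod event that mimics Superhot: world time nearly freezes while the player pawn stands still.
; Each tick it checks pawn velocity, ignored look or move input, pause, Gregory's hiding and jumpscare states, and Freddy's enter/exit transitions.
; Any of these restores normal speed; otherwise global time dilation drops sharply and the player pawn's custom dilation rises inversely to keep it at real-time speed.
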(event EventTick
  (params (DeltaSeconds :type Float%20%28single-precision%29))
  (bind _returnvalue (Game|GetPlayerController 0))
  (bind _returnvalue_2 (Game|Player|GetPlayerPawn 0))
  (bind _asgregory (Utilities|Casting|CastToGregory _returnvalue_2)
    (:then
      _)
    (:CastFailed
      _))
  (bind _asfreddy (Utilities|Casting|CastToFreddy (Class|WorldStateSystem|GetFreddyPawn (Subsystems|GetWorldStateSystem)))
    (:then
      _)
    (:CastFailed
      _))
  (if (Math|Boolean|ORBoolean (Math|Vector|NotEqual(Vector) (Transformation|GetVelocity _returnvalue_2) "0, 0, 0" 0.0001) (Class|Controller|IsLookInputIgnored _returnvalue) (Class|Controller|IsMoveInputIgnored _returnvalue) (Game|IsGamePaused) (Variables|/Game/Blueprints/Player/Gregory.Gregory_C|GetIsHiding _asgregory) (Variables|/Game/Blueprints/Player/Gregory.Gregory_C|GetIsGettingJumpScare _asgregory) (Variables|/Game/Blueprints/Player/Gregory.Gregory_C|GetHide/Unhide%20Transition%20Active _asgregory) (Variables|/Game/Blueprints/Player/Freddy.Freddy_C|GetGregoryEntering _asfreddy) (Variables|/Game/Blueprints/Player/Freddy.Freddy_C|GetGregoryExiting _asfreddy))
    (Utilities|Time|SetGlobalTimeDilation 1.0)
    (Variables|/Script/Engine.Actor|SetCustomTimeDilation _returnvalue_2 1.0)
    (else
      (Utilities|Time|SetGlobalTimeDilation 0.01)
      (Variables|/Script/Engine.Actor|SetCustomTimeDilation _returnvalue_2 1e+02))))

(fn ConstructionScript)