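; Shop location actor for ChaosMod that provides a physical button which opens the mod's shop screen.
; On BeginPlay it spawns a button actor at a fixed offset and rotation from itself and binds to its pressed event.
; When pressed, it checks the ModActor's UI state and, if none is active, sets it to the shop value and adds the Shop_Widget to the viewport.
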(event Custom|ButtonPressed
  (bind _returnvalue (Actor|GetActorOfClass "/Game/Mods/ChaosMod/ModActor.ModActor_C"))
  (if (== (Variables|/Game/Mods/ChaosMod/ModActor.ModActor_C|GetUI _returnvalue) 0)
    (Variables|/Game/Mods/ChaosMod/ModActor.ModActor_C|SetUI _returnvalue 3)
    (bind _returnvalue_2 (UserInterface|CreateWidget "/Game/Mods/ChaosMod/Content/Widgets/Shop_Widget.Shop_Widget_C"))
    (UserInterface|Viewport|AddtoViewport _returnvalue_2 998)))

(event EventBeginPlay
  (bind _returnvalue (Game|SpawnActorfromClass "/Game/Mods/ChaosMod/Content/Blueprints/ButtonActor.ButtonActor_C" (Math|Transform|MakeTransform (- (Transformation|GetActorLocation) "0,100.000000,-26.000000") "180.000000,0.000000,-90.000000" "2.000000,2.000000,2.000000") "Undefined" 0 0))
  (EventDispatchers|BindEventtoOnButtonPressed _returnvalue (delegate Custom|ButtonPressed)))

(fn ConstructionScript)