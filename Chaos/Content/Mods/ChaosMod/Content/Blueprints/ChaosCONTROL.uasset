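; ChaosMod remote-control actor for a FNAF mod: pressing 4 decodes a command hidden in an image's pixels and runs it.
; ReadData draws the texture to a render target and reads RGBA channels as a command ID plus separator-delimited ASCII arguments.
; Commands show overlay messages or images, trigger DataTable events through ModActor, set next-event text, run console commands, open URLs, kill Gregory, or change inventory.
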(event EventBeginPlay
  (bind _returnvalue (Actor|GetActorOfClass "/Game/Mods/ChaosMod/ModActor.ModActor_C"))
  (Variables|Default|SetModActor _returnvalue))

(event Input|KeyboardEvents|4
  (params (Key :type Key%20Structure :default "None"))
  (bind _returnvalue (Subsystems|GetFNAFInventorySystem))
  (bind _modactor (Variables|Default|GetModActor))
  (:Pressed
    (bind (_command _data) (CallFunction|ReadData "/Game/Mods/ChaosMod/Content/Blueprints/image.image"))
    (switch int _command
      (:0
        (bind _returnvalue_2 (UserInterface|CreateWidget "/Game/Mods/ChaosMod/Content/Widgets/Control_Overlay.Control_Overlay_C"))
        (Default|DisplayMessage _returnvalue_2 (Utilities|Text|ToText(String) (Utilities|Array|Get(acopy) _data)) (Utilities|Text|ToText(String) (Utilities|Array|Get(acopy) _data 1)) (Math|Conversions|ToFloat(Integer) (Utilities|Array|Get(acopy) _data 2)) (Math|Conversions|ToFloat(Integer) (Utilities|Array|Get(acopy) _data 3))))
      (:1
        (bind _returnvalue_3 (Utilities|GetDataTableRow "/Game/Mods/ChaosMod/Content/Blueprints/EventDataTable.EventDataTable" (Utilities|IndextoKey (Math|Conversions|ToInteger(Byte) (Utilities|Array|Get(acopy) _data))))
          (:then
            (Default|ExecuteEvent _modactor _returnvalue_3))))
      (:2
        (Development|ExecuteConsoleCommand (Utilities|Array|Get(acopy) _data) 0))
      (:3
        (CallFunction|KillGregory))
      (:4
        (Utilities|Platform|LaunchURL (Utilities|Array|Get(acopy) _data)))
      (:5
        (Rendering|Components|TextRender|SetText (Variables|/Game/Mods/ChaosMod/Content/Widgets/Overlay.Overlay_C|GetNextEventText (Variables|/Game/Mods/ChaosMod/ModActor.ModActor_C|GetOverlay _modactor)) (Utilities|Text|ToText(String) (Utilities|Array|Get(acopy) _data))))
      (:6
        (bind _returnvalue_4 (UserInterface|CreateWidget "/Game/Mods/ChaosMod/Content/Widgets/Control_Overlay.Control_Overlay_C"))
        (Default|DisplayImage _returnvalue_4 (Utilities|Array|Get(acopy) _data) (Math|Conversions|ToFloat(Integer) (Utilities|Array|Get(acopy) _data 1))))
      (:9
        (if (Utilities|Enum|Equal(Enum) (Utilities|Array|Get(acopy) _data 1) "True")
          (Class|FNAFInventorySystem|AwardItem _returnvalue (Utilities|String|StringToName (Utilities|Array|Get(acopy) _data)) true)
          (else
            (Class|FNAFInventorySystem|RemoveItem _returnvalue (Utilities|String|StringToName (Utilities|Array|Get(acopy) _data)))))))))

(fn ConstructionScript)

(fn ReadData
  (params (Texture :type Texture%20Object%20Reference))
  (bind _loc_values (LocalVariables|GetLoc_Values))
  (bind _loc_values_2 (LocalVariables|GetLoc_Values))
  (bind _loc_data (LocalVariables|GetLoc_Data))
  (bind _loc_index (LocalVariables|GetLoc_Index))
  (bind _output (Utilities|Array|Get(acopy) _loc_data _loc_index))
  (bind _returnvalue (Rendering|CreateRenderTarget2D 999 999 "RTF_RGBA16f"))
  (bind _canvas (Rendering|BeginDrawCanvastoRenderTarget _returnvalue))
  (Canvas|DrawTexture :self _canvas :RenderTexture Texture :ScreenSize "(X=180.000000,Y=1.000000)" :CoordinateSize "(X=1.000000,Y=1.000000)" :BlendMode "BLEND_Opaque" :PivotPoint "(X=0.500000,Y=0.500000)")
  (bind _index (Utilities|FlowControl|ForLoopwithBreak 0 180 :!label _label)
    (:LoopBody
      (bind _returnvalue_2 (Class|KismetRenderingLibrary|ReadRenderTargetPixel _returnvalue _index))
      (Utilities|Array|Add _loc_values (Math|Conversions|ToInteger(Byte) (.r (Math|Conversions|ToColor(LinearColor) (Math|Conversions|ToLinearColor(Color) _returnvalue_2)))))
      (Utilities|Array|Add _loc_values (Math|Conversions|ToInteger(Byte) (.g (Math|Conversions|ToColor(LinearColor) (Math|Conversions|ToLinearColor(Color) _returnvalue_2)))))
      (Utilities|Array|Add _loc_values (Math|Conversions|ToInteger(Byte) (.b (Math|Conversions|ToColor(LinearColor) (Math|Conversions|ToLinearColor(Color) _returnvalue_2)))))
      (Utilities|Array|Add _loc_values (Math|Conversions|ToInteger(Byte) (.a (Math|Conversions|ToColor(LinearColor) (Math|Conversions|ToLinearColor(Color) _returnvalue_2)))))
      (if (Math|Boolean|ORBoolean (== (Math|Conversions|ToInteger(Byte) (.r (Math|Conversions|ToColor(LinearColor) (Math|Conversions|ToLinearColor(Color) _returnvalue_2)))) 31) (== (Math|Conversions|ToInteger(Byte) (.g (Math|Conversions|ToColor(LinearColor) (Math|Conversions|ToLinearColor(Color) _returnvalue_2)))) 31) (== (Math|Conversions|ToInteger(Byte) (.b (Math|Conversions|ToColor(LinearColor) (Math|Conversions|ToLinearColor(Color) _returnvalue_2)))) 31) (== (Math|Conversions|ToInteger(Byte) (.a (Math|Conversions|ToColor(LinearColor) (Math|Conversions|ToLinearColor(Color) _returnvalue_2)))) 31))
        (goto _label Break)))
    (:Completed
      (LocalVariables|SetLoc_Command (Utilities|Array|Get(acopy) _loc_values_2))
      (Utilities|Array|RemoveIndex _loc_values_2)
      (for _array_element _loc_values_2
        (if (== _array_element 30)
          (Math|Integer|IncrementInt _loc_index)
          (else
            (|SetBy-RefVar _output (Utilities|String|Append _output (Utilities|Array|Get(acopy) (LocalVariables|GetLoc_ASCII) _array_element))))))
      (return (LocalVariables|GetLoc_Command) (LocalVariables|GetLoc_Data)))))