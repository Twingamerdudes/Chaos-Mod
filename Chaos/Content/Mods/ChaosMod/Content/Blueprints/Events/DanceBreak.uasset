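; DanceBreak is a ChaosMod event Blueprint that shows the DanceBreak widget, with webcam support when a capture device is available.
; On BeginPlay it enumerates video capture devices and opens the first URL in media player MP, before checking whether the list is empty.
; When media opens it adds the widget with Wc true; with no devices it adds it with Wc false.
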(event Custom|OnMediaOpened
  (params (OpenedUrl :type String))
  (bind _returnvalue (UserInterface|CreateWidget "/Game/Mods/ChaosMod/Content/Widgets/Events/DanceBreak.DanceBreak_C" 0 true))
  (UserInterface|Viewport|AddtoViewport _returnvalue 0))

(event EventBeginPlay
  (bind _mp (Variables|Default|GetMP))
  (bind _outdevices (Class|MediaBlueprintFunctionLibrary|EnumerateVideoCaptureDevices (|BitmaskLiteral 15)))
  (EventDispatchers|AssignOnMediaOpened _mp (delegate Custom|OnMediaOpened))
  (Class|MediaPlayer|OpenUrl _mp (.url (Utilities|Array|Get(acopy) _outdevices)))
  (if (== (Utilities|Array|Length _outdevices) 0)
    (bind _returnvalue (UserInterface|CreateWidget "/Game/Mods/ChaosMod/Content/Widgets/Events/DanceBreak.DanceBreak_C"))
    (UserInterface|Viewport|AddtoViewport _returnvalue 0)))

(fn ConstructionScript)