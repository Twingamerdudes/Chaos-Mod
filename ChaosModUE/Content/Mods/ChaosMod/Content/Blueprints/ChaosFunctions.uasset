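; ChaosMod helper functions for gathering enemies and roughly alphabetizing string arrays.
; GetAllEnemies combines StaffBotSecurityPatrol and MapBot actors with all AI registered in the AI management system, without removing duplicates.
; SortArrayOfStrings is a single-pass, case-insensitive bucket sort on the character at StartIndex, using a long if-chain.
; It joins buckets A to Z, puts anything else last, and keeps input order within each bucket.
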(fn GetAllEnemies
  (bind _loc_enemies (LocalVariables|GetLoc_Enemies))
  (bind _outactors (Actor|GetAllActorsOfClass 0 "/Game/Blueprints/AI/StaffBot/Security/Patrol/StaffBotSecurityPatrol.StaffBotSecurityPatrol_C"))
  (bind _outactors_2 (Actor|GetAllActorsOfClass 0 "/Game/Blueprints/AI/StaffBot/MapBot/MapBot.MapBot_C"))
  (Utilities|Array|AppendArray _loc_enemies _outactors)
  (Utilities|Array|AppendArray _loc_enemies _outactors_2)
  (Utilities|Array|AppendArray _loc_enemies (Class|AIManagementSystem|GetAllRegisteredAI (Subsystems|GetAIManagementSystem)))
  (return _loc_enemies))

(fn SortArrayOfStrings
  (params (Array :type Array%20of%20Strings) (StartIndex :type Integer))
  (bind _returnvalue (Utilities|Array|Length Array))
  (bind _a (LocalVariables|GetA))
  (bind _b (LocalVariables|GetB))
  (bind _e (LocalVariables|GetE))
  (bind _k (LocalVariables|GetK))
  (bind _l (LocalVariables|GetL))
  (bind _m (LocalVariables|GetM))
  (bind _n (LocalVariables|GetN))
  (bind _o (LocalVariables|GetO))
  (bind _p (LocalVariables|GetP))
  (bind _q (LocalVariables|GetQ))
  (bind _r (LocalVariables|GetR))
  (bind _s (LocalVariables|GetS))
  (bind _c (LocalVariables|GetC))
  (bind _t (LocalVariables|GetT))
  (bind _u (LocalVariables|GetU))
  (bind _v (LocalVariables|GetV))
  (bind _w (LocalVariables|GetW))
  (bind _x (LocalVariables|GetX))
  (bind _y (LocalVariables|GetY))
  (bind _z (LocalVariables|GetZ))
  (bind _other (LocalVariables|Getother))
  (bind _sortedarray (LocalVariables|GetSortedArray))
  (bind _d (LocalVariables|GetD))
  (bind _j (LocalVariables|GetJ))
  (bind _f (LocalVariables|GetF))
  (bind _g (LocalVariables|GetG))
  (bind _h (LocalVariables|GetH))
  (bind _i (LocalVariables|GetI))
  (bind _returnvalue_2 (> _returnvalue 1))
  (if _returnvalue_2
    (for _array_element Array
      (if (Utilities|Enum|Equal(Enum) (Utilities|String|GetSubstring (Class|KismetStringLibrary|ToUpper _array_element) StartIndex) "A")
        (Utilities|Array|Add _a _array_element)
        (elif (Utilities|Enum|Equal(Enum) (Utilities|String|GetSubstring (Class|KismetStringLibrary|ToUpper _array_element) StartIndex) "B")
          (Utilities|Array|Add _b _array_element)
          (elif (Utilities|Enum|Equal(Enum) (Utilities|String|GetSubstring (Class|KismetStringLibrary|ToUpper _array_element) StartIndex) "C")
            (Utilities|Array|Add _c _array_element)
            (elif (Utilities|Enum|Equal(Enum) (Utilities|String|GetSubstring (Class|KismetStringLibrary|ToUpper _array_element) StartIndex) "D")
              (Utilities|Array|Add _d _array_element)
              (elif (Utilities|Enum|Equal(Enum) (Utilities|String|GetSubstring (Class|KismetStringLibrary|ToUpper _array_element) StartIndex) "E")
                (Utilities|Array|Add _e _array_element)
                (elif (Utilities|Enum|Equal(Enum) (Utilities|String|GetSubstring (Class|KismetStringLibrary|ToUpper _array_element) StartIndex) "F")
                  (Utilities|Array|Add _f _array_element)
                  (elif (Utilities|Enum|Equal(Enum) (Utilities|String|GetSubstring (Class|KismetStringLibrary|ToUpper _array_element) StartIndex) "G")
                    (Utilities|Array|Add _g _array_element)
                    (elif (Utilities|Enum|Equal(Enum) (Utilities|String|GetSubstring (Class|KismetStringLibrary|ToUpper _array_element) StartIndex) "H")
                      (Utilities|Array|Add _h _array_element)
                      (elif (Utilities|Enum|Equal(Enum) (Utilities|String|GetSubstring (Class|KismetStringLibrary|ToUpper _array_element) StartIndex) "I")
                        (Utilities|Array|Add _i _array_element)
                        (elif (Utilities|Enum|Equal(Enum) (Utilities|String|GetSubstring (Class|KismetStringLibrary|ToUpper _array_element) StartIndex) "J")
                          (Utilities|Array|Add _j _array_element)
                          (elif (Utilities|Enum|Equal(Enum) (Utilities|String|GetSubstring (Class|KismetStringLibrary|ToUpper _array_element) StartIndex) "K")
                            (Utilities|Array|Add _k _array_element)
                            (elif (Utilities|Enum|Equal(Enum) (Utilities|String|GetSubstring (Class|KismetStringLibrary|ToUpper _array_element) StartIndex) "L")
                              (Utilities|Array|Add _l _array_element)
                              (elif (Utilities|Enum|Equal(Enum) (Utilities|String|GetSubstring (Class|KismetStringLibrary|ToUpper _array_element) StartIndex) "M")
                                (Utilities|Array|Add _m _array_element)
                                (elif (Utilities|Enum|Equal(Enum) (Utilities|String|GetSubstring (Class|KismetStringLibrary|ToUpper _array_element) StartIndex) "N")
                                  (Utilities|Array|Add _n _array_element)
                                  (elif (Utilities|Enum|Equal(Enum) (Utilities|String|GetSubstring (Class|KismetStringLibrary|ToUpper _array_element) StartIndex) "O")
                                    (Utilities|Array|Add _o _array_element)
                                    (elif (Utilities|Enum|Equal(Enum) (Utilities|String|GetSubstring (Class|KismetStringLibrary|ToUpper _array_element) StartIndex) "P")
                                      (Utilities|Array|Add _p _array_element)
                                      (elif (Utilities|Enum|Equal(Enum) (Utilities|String|GetSubstring (Class|KismetStringLibrary|ToUpper _array_element) StartIndex) "Q")
                                        (Utilities|Array|Add _q _array_element)
                                        (elif (Utilities|Enum|Equal(Enum) (Utilities|String|GetSubstring (Class|KismetStringLibrary|ToUpper _array_element) StartIndex) "R")
                                          (Utilities|Array|Add _r _array_element)
                                          (elif (Utilities|Enum|Equal(Enum) (Utilities|String|GetSubstring (Class|KismetStringLibrary|ToUpper _array_element) StartIndex) "S")
                                            (Utilities|Array|Add _s _array_element)
                                            (elif (Utilities|Enum|Equal(Enum) (Utilities|String|GetSubstring (Class|KismetStringLibrary|ToUpper _array_element) StartIndex) "T")
                                              (Utilities|Array|Add _t _array_element)
                                              (elif (Utilities|Enum|Equal(Enum) (Utilities|String|GetSubstring (Class|KismetStringLibrary|ToUpper _array_element) StartIndex) "U")
                                                (Utilities|Array|Add _u _array_element)
                                                (elif (Utilities|Enum|Equal(Enum) (Utilities|String|GetSubstring (Class|KismetStringLibrary|ToUpper _array_element) StartIndex) "V")
                                                  (Utilities|Array|Add _v _array_element)
                                                  (elif (Utilities|Enum|Equal(Enum) (Utilities|String|GetSubstring (Class|KismetStringLibrary|ToUpper _array_element) StartIndex) "W")
                                                    (Utilities|Array|Add _w _array_element)
                                                    (elif (Utilities|Enum|Equal(Enum) (Utilities|String|GetSubstring (Class|KismetStringLibrary|ToUpper _array_element) StartIndex) "X")
                                                      (Utilities|Array|Add _x _array_element)
                                                      (elif (Utilities|Enum|Equal(Enum) (Utilities|String|GetSubstring (Class|KismetStringLibrary|ToUpper _array_element) StartIndex) "Y")
                                                        (Utilities|Array|Add _y _array_element)
                                                        (elif (Utilities|Enum|Equal(Enum) (Utilities|String|GetSubstring (Class|KismetStringLibrary|ToUpper _array_element) StartIndex) "Z")
                                                          (Utilities|Array|Add _z _array_element)
                                                          (else
                                                            (Utilities|Array|Add _other _array_element)))))))))))))))))))))))))))))
    (Utilities|Array|AppendArray _sortedarray _a)
    (Utilities|Array|AppendArray _sortedarray _b)
    (Utilities|Array|AppendArray _sortedarray _c)
    (Utilities|Array|AppendArray _sortedarray _d)
    (Utilities|Array|AppendArray _sortedarray _e)
    (Utilities|Array|AppendArray _sortedarray _f)
    (Utilities|Array|AppendArray _sortedarray _g)
    (Utilities|Array|AppendArray _sortedarray _h)
    (Utilities|Array|AppendArray _sortedarray _i)
    (Utilities|Array|AppendArray _sortedarray _j)
    (Utilities|Array|AppendArray _sortedarray _k)
    (Utilities|Array|AppendArray _sortedarray _l)
    (Utilities|Array|AppendArray _sortedarray _m)
    (Utilities|Array|AppendArray _sortedarray _n)
    (Utilities|Array|AppendArray _sortedarray _o)
    (Utilities|Array|AppendArray _sortedarray _p)
    (Utilities|Array|AppendArray _sortedarray _q)
    (Utilities|Array|AppendArray _sortedarray _r)
    (Utilities|Array|AppendArray _sortedarray _s)
    (Utilities|Array|AppendArray _sortedarray _t)
    (Utilities|Array|AppendArray _sortedarray _u)
    (Utilities|Array|AppendArray _sortedarray _v)
    (Utilities|Array|AppendArray _sortedarray _w)
    (Utilities|Array|AppendArray _sortedarray _x)
    (Utilities|Array|AppendArray _sortedarray _y)
    (Utilities|Array|AppendArray _sortedarray _z)
    (Utilities|Array|AppendArray _sortedarray _other))
  (return (select _returnvalue_2 _sortedarray Array)))