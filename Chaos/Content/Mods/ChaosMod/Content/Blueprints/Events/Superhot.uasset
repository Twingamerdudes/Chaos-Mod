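; Chaos mod event that mimics Superhot: time nearly freezes while the player pawn stands still.
; Each tick it sets global time dilation to normal or near zero based on player velocity, with inverse pawn dilation keeping the player at full speed.
; Gregory's hiding, hide transitions and jumpscares, and Gregory entering or exiting Freddy, also keep time normal, read from actors cached at BeginPlay.
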(event EventBeginPlay
  (bind _returnvalue (Actor|GetActorOfClass "/Game/Blueprints/Player/Freddy.Freddy_C"))
  (bind _returnvalue_2 (Actor|GetActorOfClass "/Game/Blueprints/Player/Gregory.Gregory_C")))

(event EventTick
  (params (DeltaSeconds :type Float%20%28single-precision%29))
  (bind _returnvalue (Game|Player|GetPlayerPawn 0))
  (if (Math|Boolean|ORBoolean (Math|Vector|NotEqual(Vector) (Transformation|GetVelocity _returnvalue) "0, 0, 0" 0.0001) (Variables|/Game/Blueprints/Player/Gregory.Gregory_C|GetIsHiding (stale EventBeginPlay _returnvalue_2)) (Variables|/Game/Blueprints/Player/Gregory.Gregory_C|GetIsGettingJumpScare (stale EventBeginPlay _returnvalue_2)) (Variables|/Game/Blueprints/Player/Gregory.Gregory_C|GetHide/Unhide%20Transition%20Active (stale EventBeginPlay _returnvalue_2)) (Variables|/Game/Blueprints/Player/Freddy.Freddy_C|GetGregoryEntering (stale EventBeginPlay _returnvalue)) (Variables|/Game/Blueprints/Player/Freddy.Freddy_C|GetGregoryExiting (stale EventBeginPlay _returnvalue)))
    (Utilities|Time|SetGlobalTimeDilation 1.0)
    (Variables|/Script/Engine.Actor|SetCustomTimeDilation _returnvalue 1.0)
    (else
      (Utilities|Time|SetGlobalTimeDilation 0.01)
      (Variables|/Script/Engine.Actor|SetCustomTimeDilation _returnvalue 1e+02))))

(fn ConstructionScript)