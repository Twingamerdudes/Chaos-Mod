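; Shop location actor for ChaosMod that opens the shop and runs effects of its item flags.
; BeginPlay spawns a hidden BasicToggleButton, which Tick polls to show Shop_Widget when no ModActor UI is active.
; Tick also drives Item 3, repeatedly halving enemy CustomTimeDilation per class, and Item 4, auto-recharging the Fazerblaster and Fazcam.
; With Item 5, G toggles gun storage by destroying or respawning the Gun actor.
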(event EventBeginPlay
  ;[1 1 1] Setup
  (bind _returnvalue (Game|SpawnActorfromClass "/Game/Blueprints/Button/BasicToggleButton.BasicToggleButton_C" (Math|Transform|MakeTransform (- (Transformation|GetActorLocation) "0,136.000000,-80.000000") "0, 0, 0" "10.000000,1.000000,1.000000") "Undefined" 0 0))
  (bind _output_get (Variables|Default|SetButton _returnvalue))
  (Utilities|FlowControl|Sequence
    (:then_0
      (bind _returnvalue_2 (Actor|GetActorOfClass "/Game/Mods/ChaosMod/ModActor.ModActor_C"))
      (Variables|Default|SetModActor _returnvalue_2)
      (bind _returnvalue_3 (Actor|GetActorOfClass "/Game/Blueprints/Objects/Equippables/EQ_LaserGun.EQ_LaserGun_C"))
      (Variables|Default|SetFazerblaster _returnvalue_3))
    (:then_1
      (Rendering|SetActorHiddenInGame _output_get true)
      (bind _returnvalue_4 (Actor|GetActorOfClass "/Game/Blueprints/Objects/Equippables/EQ_Flashbeacon.EQ_Flashbeacon_C"))
      (Variables|Default|SetFazcam _returnvalue_4))))

(event EventTick
  (params (DeltaSeconds :type Float%20%28single-precision%29))
  (bind _fazcam (Variables|Default|GetFazcam))
  (bind _button (Variables|Default|GetButton))
  (bind _modactor (Variables|Default|GetModActor))
  (bind _fazerblaster (Variables|Default|GetFazerblaster))
  ;[1 1 1] Button
  (Utilities|FlowControl|Sequence
    (:then_0
      (if (Variables|/Game/Blueprints/Button/BasicToggleButton.BasicToggleButton_C|GetState _button)
        (if (== (Variables|/Game/Mods/ChaosMod/ModActor.ModActor_C|GetUI _modactor) 0)
          (Variables|/Game/Mods/ChaosMod/ModActor.ModActor_C|SetUI _modactor 3)
          (bind _returnvalue (UserInterface|CreateWidget "/Game/Mods/ChaosMod/Content/Widgets/Shop_Widget.Shop_Widget_C"))
          (UserInterface|Viewport|AddtoViewport _returnvalue 998))
        (Variables|/Game/Blueprints/Button/BasicToggleButton.BasicToggleButton_C|SetState _button false)))
    (:then_1
      ;[1 1 1] Item 3
      (if (Variables|Default|GetItem%203)
        (Utilities|FlowControl|Delay 2.0)
        (Utilities|EnemyDilation 0.5)))
    (:then_2
      ;[1 1 1] Item 4
      (if (Variables|Default|GetItem%204)
        (Utilities|FlowControl|Sequence
          (:then_0
            (if (<= (Variables|/Game/Blueprints/Objects/Equippables/EQ_LaserGun.EQ_LaserGun_C|GetShotsLeft _fazerblaster) 5)
              (Default|Recharge _fazerblaster)))
          (:then_1
            (if (not (Variables|/Game/Blueprints/Objects/Equippables/EQ_Flashbeacon.EQ_Flashbeacon_C|GetCanUse? _fazcam))
              (Utilities|FlowControl|DoOnce false :!label _label
                (:Completed
                  (Default|Recharging _fazcam)
                  (Utilities|FlowControl|Delay 1.2)
                  (goto _label Reset))))))))))

(event Input|KeyboardEvents|G
  (params (Key :type Key%20Structure :default "None"))
  ;[1 1 1] Item 5
  (:Pressed
    (if (Variables|Default|GetItem%205)
      (if (Variables|Default|GetGun%20Stored)
        (Variables|Default|SetGun%20Stored false)
        (Game|SpawnActorfromClass "/Game/Mods/ChaosMod/Content/Blueprints/Events/Gun.Gun_C" (Math|Conversions|ToTransform(Vector) "0, 0, 0") "Undefined" 0 0)
        (else
          (Variables|Default|SetGun%20Stored true)
          (bind _returnvalue (Actor|GetActorOfClass "/Game/Mods/ChaosMod/Content/Blueprints/Events/Gun.Gun_C"))
          (Actor|DestroyActor _returnvalue))))))

(fn ConstructionScript)