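; Chaos mod event actor that follows the player around as a set of static meshes, named as grass.
; On BeginPlay it gives each static mesh component a random yaw, keeping pitch and roll.
; Each Tick it interpolates toward player character 0 at a speed equal to the capped distance, so it eases off when close.
; The interpolated point is projected onto the navmesh before the actor moves there without sweeping.
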(event EventBeginPlay
  (for _array_element (Actor|GetComponentsByClass "/Script/Engine.StaticMeshComponent")
    (Transformation|SetWorldRotation _array_element (Math|Rotator|MakeRotator (.roll (Transformation|GetWorldRotation _array_element)) (.pitch (Transformation|GetWorldRotation _array_element)) (Math|Random|RandomFloatinRange 0.0 3.6e+02)) false false)))

(event EventTick
  (params (DeltaSeconds :type Float%20%28single-precision%29))
  (bind _returnvalue (Game|GetPlayerCharacter 0))
  (bind _returnvalue_2 (Transformation|GetActorLocation))
  (bind _returnvalue_3 (Transformation|GetActorLocation _returnvalue))
  (Transformation|SetActorLocation (.ProjectedLocation (AI|Navigation|ProjectPointtoNavigation (Math|Interpolation|VInterpTo _returnvalue_2 _returnvalue_3 DeltaSeconds (Math|Float|Clamp(Float) (Math|Vector|Distance(Vector) _returnvalue_2 _returnvalue_3) 0.0 6.0)) 0 0 "500.000000,500.000000,500.000000")) false false))

(fn ConstructionScript)