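; Chaos Mod event actor that shadows a hidden Montgomery Gator AI, apparently to pursue Gregory.
; On BeginPlay it spawns MontyStandard, hides it, runs the MontyShowtimeBT behavior tree and tunes its movement speed and acceleration.
; Each Tick it issues an AI move toward Gregory, with no pawn shown on the call, and teleports itself onto the hidden Monty, using it as a movement proxy.
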(event EventBeginPlay
  (bind _returnvalue (Game|SpawnActorfromClass "/Game/Blueprints/AI/Seeker/Monty/MontyStandard.MontyStandard_C" (Transformation|GetActorTransform) "Undefined" 0 0))
  (AI|RunBehaviorTree (AI|GetAIController _returnvalue) "/Game/Blueprints/AI/Seeker/Monty/MontyShowtime/MontyShowtimeBT.MontyShowtimeBT")
  (Rendering|SetActorHiddenInGame _returnvalue true)
  (bind _returnvalue_2 (Actor|GetActorOfClass "/Game/Blueprints/Player/Gregory.Gregory_C"))
  (Variables|/Script/Engine.CharacterMovementComponent|SetMaxWalkSpeed (Variables|/Script/Engine.Character|GetCharacterMovement _returnvalue) 1e+03)
  (Variables|/Script/Engine.CharacterMovementComponent|SetMaxAcceleration (Variables|/Script/Engine.Character|GetCharacterMovement _returnvalue) 2.5e+02))

(event EventTick
  (params (DeltaSeconds :type Float%20%28single-precision%29))
  (Utilities|FlowControl|Sequence
    (:then_0
      (AI|AIMoveTo 0 (Transformation|GetActorLocation (stale EventBeginPlay _returnvalue_2)) 0 5.0 false))
    (:then_1
      (Transformation|Teleport (Transformation|GetActorLocation (stale EventBeginPlay _returnvalue)) "0, 0, 0"))))

(fn ConstructionScript)