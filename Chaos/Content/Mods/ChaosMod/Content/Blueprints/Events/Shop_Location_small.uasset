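; Small shop location for ChaosMod that opens the shop UI when its button is toggled.
; On BeginPlay it spawns a hidden, X-stretched BasicToggleButton at a fixed world position and caches the ModActor.
; Tick polls and resets the button state, adding a Shop_Widget to the viewport only when ModActor's UI state is free, then marking that state as occupied.
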(event EventBeginPlay
  ;[1 1 1] Setup
  (bind _returnvalue (Game|SpawnActorfromClass "/Game/Blueprints/Button/BasicToggleButton.BasicToggleButton_C" (Math|Transform|MakeTransform "-1700.000000,31764.000000,2155.000000" "0, 0, 0" "10.000000,1.000000,1.000000") "Undefined" 0 0))
  (bind _output_get (Variables|Default|SetButton _returnvalue))
  (Rendering|SetActorHiddenInGame _output_get true)
  (bind _returnvalue_2 (Actor|GetActorOfClass "/Game/Mods/ChaosMod/ModActor.ModActor_C"))
  (Variables|Default|SetModActor _returnvalue_2))

(event EventTick
  (params (DeltaSeconds :type Float%20%28single-precision%29))
  (bind _button (Variables|Default|GetButton))
  (bind _modactor (Variables|Default|GetModActor))
  ;[1 1 1] Button
  (if (Variables|/Game/Blueprints/Button/BasicToggleButton.BasicToggleButton_C|GetState _button)
    (if (== (Variables|/Game/Mods/ChaosMod/ModActor.ModActor_C|GetUI _modactor) 0)
      (Variables|/Game/Mods/ChaosMod/ModActor.ModActor_C|SetUI _modactor 3)
      (bind _returnvalue (UserInterface|CreateWidget "/Game/Mods/ChaosMod/Content/Widgets/Shop_Widget.Shop_Widget_C"))
      (UserInterface|Viewport|AddtoViewport _returnvalue 998))
    (Variables|/Game/Blueprints/Button/BasicToggleButton.BasicToggleButton_C|SetState _button false)))

(fn ConstructionScript)