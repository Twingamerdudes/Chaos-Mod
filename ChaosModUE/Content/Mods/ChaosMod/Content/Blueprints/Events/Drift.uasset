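; Drift is a Chaos Mod event that makes the player's view slowly drift in a random direction.
; On BeginPlay it picks small random pitch and yaw offsets, each either positive or negative.
; Every Tick it adds those fixed offsets to the first player's control rotation, keeping roll unchanged.
; The offsets are not scaled by delta time, so drift speed depends on frame rate.
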(event EventBeginPlay
  (bind _returnvalue (Math|Random|RandomFloatinRange -0.2 0.2))
  (Variables|Default|SetY _returnvalue)
  (Variables|Default|SetZ _returnvalue))

(event EventTick
  (params (DeltaSeconds :type Float%20%28single-precision%29))
  (bind _returnvalue (Game|GetPlayerCharacter 0))
  (bind _returnvalue_2 (Pawn|GetControlRotation _returnvalue :!class /Script/Engine.Pawn))
  (Pawn|SetControlRotation (Game|GetPlayerController 0) (Math|Rotator|MakeRotator (.roll _returnvalue_2) (+ (.pitch _returnvalue_2) (Variables|Default|GetY)) (+ (.yaw _returnvalue_2) (Variables|Default|GetZ)))))

(fn ConstructionScript)