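; FazGlock is a Chaos Mod pistol actor that lets Gregory shoot animatronics, with input ignored while inside Freddy.
; Key 4 toggles it via actor visibility and item swapping, keys 1–3 holster it for owned items, and an Overlay flag follows.
; Firing spends ammo, makes noise, shakes the camera and line-traces, destroying registered AI or StaffBots and pushing movable components.
; R reloads after a timed animation; traces leave persistent debug lines.
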(event EventBeginPlay
  (bind _foundwidgets (Widget|GetAllWidgetsOfClass "/Game/Mods/ChaosMod/Content/Widgets/Overlay.Overlay_C" true))
  (bind _output_get (Variables|Default|SetOverlay (Utilities|Array|Get(acopy) _foundwidgets)))
  (Variables|/Game/Mods/ChaosMod/Content/Widgets/Overlay.Overlay_C|SetGun _output_get true))

(event Input|MouseEvents|LeftMouseButton
  (params (Key :type Key%20Structure))
  (bind _returnvalue (Game|Player|GetPlayerPawn 0))
  (bind _returnvalue_2 (Game|GetPlayerCameraManager 0))
  (bind _ammo (Variables|Default|GetAmmo))
  (bind _returnvalue_3 (Transformation|GetActorForwardVector _returnvalue_2))
  (bind _returnvalue_4 (Camera|GetCameraLocation _returnvalue_2))
  (bind _returnvalue_5 (* _returnvalue_3 100000))
  (:Pressed
    (if (Math|Boolean|ANDBoolean (not (Variables|Default|GetReloading)) (not (Variables|Rendering|GetbHidden)) (not (Class|WorldStateSystem|IsPlayerinFreddy (Subsystems|GetWorldStateSystem))))
      (Utilities|DoOnce(selfReset) false 0.1)
      (if (> _ammo 0)
        (Math|Integer|DecrementInt _ammo
          (:%20%20
            (Components|Animation|PlayAnimation (Variables|Default|GetSkeletalMesh) "/Game/Mods/ChaosMod/Content/Models/Fire_Pistol_W.Fire_Pistol_W" false)
            (Class|Actor|MakeNoise 1e+01 _returnvalue (Transformation|GetActorLocation _returnvalue) 1e+04 "None")
            (Camera|PlayWorldCameraShake "/Game/Mods/ChaosMod/Content/Blueprints/ShootingMaShot.ShootingMaShot_C" _returnvalue_4 5e+01 1e+01)
            (bind (_outhit _returnvalue_6) (Collision|LineTraceByChannel _returnvalue_4 (+ _returnvalue_4 _returnvalue_5) "TraceTypeQuery2" true (Utilities|Array|MakeArray (Game|Player|GetPlayerPawn 0)) "Persistent"))
            (if _returnvalue_6
              (bind _aspawn (Utilities|Casting|CastToPawn (.HitActor (Collision|BreakHitResult _outhit)))
                (:then
                  (if (Utilities|Array|ContainsItem (Class|AIManagementSystem|GetAllRegisteredAI (Subsystems|GetAIManagementSystem)) _aspawn)
                    (Actor|DestroyActor _aspawn)
                    (else
                      (bind _asstaff_bot_base (Utilities|Casting|CastToStaffBotBase _aspawn))
                      (Actor|DestroyActor _asstaff_bot_base))))
                (:CastFailed
                  (switch Utilities|FlowControl|Switch|SwitchonEComponentMobility (Variables|/Script/Engine.SceneComponent|GetMobility (.HitComponent (Collision|BreakHitResult _outhit)))
                    (:Movable
                      (Physics|AddImpulse (.HitComponent (Collision|BreakHitResult _outhit)) (/ _returnvalue_5 100) "None" true))))))))
        (else
          (Audio|PlaySound2D "/Game/Mods/ChaosMod/Content/Audio/Pistol_ReloadMagInsert01.Pistol_ReloadMagInsert01" 1.0 1.0 0.0 0 0))))))

(event Input|KeyboardEvents|R
  (params (Key :type Key%20Structure))
  (:Pressed
    (if (Math|Boolean|ANDBoolean (not (Variables|Default|GetReloading)) (not (Variables|Rendering|GetbHidden)) (< (Variables|Default|GetAmmo) 9) (not (Class|WorldStateSystem|IsPlayerinFreddy (Subsystems|GetWorldStateSystem))))
      (Variables|Default|SetReloading true)
      (Components|Animation|PlayAnimation (Variables|Default|GetSkeletalMesh) "/Game/Mods/ChaosMod/Content/Models/Reload_Pistol_W.Reload_Pistol_W" false)
      (Utilities|FlowControl|Delay 1.7)
      (Variables|Default|SetAmmo 9)
      (Variables|Default|SetReloading false))))

(event Input|KeyboardEvents|4
  (params (Key :type Key%20Structure))
  (bind _overlay (Variables|Default|GetOverlay))
  (:Pressed
    (if (not (Class|WorldStateSystem|IsPlayerinFreddy (Subsystems|GetWorldStateSystem)))
      (bind _asgregory (Utilities|Casting|CastToGregory (Game|GetPlayerCharacter 0)))
      (if (Variables|Rendering|GetbHidden)
        (Variables|Default|SetItem (Variables|/Game/Blueprints/Player/Gregory.Gregory_C|GetEquippedItem _asgregory))
        (Default|SwitchItemwithAnim _asgregory)
        (Variables|/Game/Mods/ChaosMod/Content/Widgets/Overlay.Overlay_C|SetGun _overlay true)
        (Utilities|FlowControl|Delay 0.4)
        (Rendering|SetActorHiddenInGame false)
        (else
          (Variables|/Game/Blueprints/Player/Gregory.Gregory_C|SetEquippedItem _asgregory (Variables|Default|GetItem))
          (Variables|/Game/Mods/ChaosMod/Content/Widgets/Overlay.Overlay_C|SetGun _overlay false)
          (Rendering|SetActorHiddenInGame true))))))

(event Input|KeyboardEvents|3
  (params (Key :type Key%20Structure))
  (:Pressed
    (if (and (Class|FNAFInventorySystem|HasItem (Subsystems|GetFNAFInventorySystem) "FlashBeacon") (not (Class|WorldStateSystem|IsPlayerinFreddy (Subsystems|GetWorldStateSystem))))
      (Rendering|SetActorHiddenInGame true)
      (Variables|/Game/Mods/ChaosMod/Content/Widgets/Overlay.Overlay_C|SetGun (Variables|Default|GetOverlay) false))))

(event Input|KeyboardEvents|2
  (params (Key :type Key%20Structure))
  (:Pressed
    (if (and (Class|FNAFInventorySystem|HasItem (Subsystems|GetFNAFInventorySystem) "Fazergun") (not (Class|WorldStateSystem|IsPlayerinFreddy (Subsystems|GetWorldStateSystem))))
      (Rendering|SetActorHiddenInGame true)
      (Variables|/Game/Mods/ChaosMod/Content/Widgets/Overlay.Overlay_C|SetGun (Variables|Default|GetOverlay) false))))

(event Input|KeyboardEvents|1
  (params (Key :type Key%20Structure))
  (:Pressed
    (if (and (Class|FNAFInventorySystem|HasItem (Subsystems|GetFNAFInventorySystem) "Flashlight") (not (Class|WorldStateSystem|IsPlayerinFreddy (Subsystems|GetWorldStateSystem))))
      (Rendering|SetActorHiddenInGame true)
      (Variables|/Game/Mods/ChaosMod/Content/Widgets/Overlay.Overlay_C|SetGun (Variables|Default|GetOverlay) false))))

(fn ConstructionScript)