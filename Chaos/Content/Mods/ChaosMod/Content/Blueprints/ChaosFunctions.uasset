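; ChaosFunctions holds shared helper functions for the ChaosMod mod, covering player death and enemy lookup.
; KillGregory calls EjectGregory on the first Freddy and Burntrap_Freddy actors found, then calls Kill on the Gregory actor.
; GetAllEnemies returns one array combining all security patrol StaffBots, all MapBots and every AI registered with the AIManagementSystem.
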(fn KillGregory
  (bind _returnvalue (Actor|GetActorOfClass 0 "/Game/Blueprints/Player/Freddy.Freddy_C"))
  (Default|EjectGregory _returnvalue)
  (bind _returnvalue_2 (Actor|GetActorOfClass 0 "/Game/Blueprints/Player/Burntrap_Freddy.Burntrap_Freddy_C"))
  (Default|EjectGregory _returnvalue_2)
  (bind _returnvalue_3 (Actor|GetActorOfClass 0 "/Game/Blueprints/Player/Gregory.Gregory_C"))
  (Default|Kill _returnvalue_3)
  (return))

(fn GetAllEnemies
  (bind _loc_enemies (LocalVariables|GetLoc_Enemies))
  (bind _outactors (Actor|GetAllActorsOfClass 0 "/Game/Blueprints/AI/StaffBot/Security/Patrol/StaffBotSecurityPatrol.StaffBotSecurityPatrol_C"))
  (bind _outactors_2 (Actor|GetAllActorsOfClass 0 "/Game/Blueprints/AI/StaffBot/MapBot/MapBot.MapBot_C"))
  (Utilities|Array|AppendArray _loc_enemies _outactors)
  (Utilities|Array|AppendArray _loc_enemies _outactors_2)
  (Utilities|Array|AppendArray _loc_enemies (Class|AIManagementSystem|GetAllRegisteredAI (Subsystems|GetAIManagementSystem)))
  (return _loc_enemies))