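; Chaos mod event actor that plays a Wobble sound alongside a screen wobble post-process effect.
; On BeginPlay it adds a dynamic PP_Wobble material instance to the ModActor's post-process settings.
; Tick increments the material's "x" parameter by a fixed step per frame, while chained delays reset it three times at equal intervals.
; When the sound finishes, it removes the material and destroys itself.
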(event Custom|OnAudioFinished
  (Utilities|Array|RemoveItem (.array (Utilities|Struct|BreakPostProcessSettings (Variables|/Script/Engine.PostProcessComponent|GetSettings (Variables|/Game/Mods/ChaosMod/ModActor.ModActor_C|GetPostProcess (Variables|Default|GetModActor))))) (Utilities|Struct|MakeWeightedBlendable 1.0 (stale EventBeginPlay _returnvalue_3)))
  (Actor|DestroyActor))

(event EventTick
  (params (DeltaSeconds :type Float%20%28single-precision%29))
  (bind _output_get (Variables|Default|Setx (+ (Variables|Default|Getx) 0.1)))
  (Rendering|Material|SetScalarParameterValue (stale EventBeginPlay _returnvalue_3) "x" _output_get :!class /Script/Engine.MaterialInstanceDynamic))

(event EventBeginPlay
  (bind _returnvalue (Actor|GetActorOfClass "/Game/Mods/ChaosMod/ModActor.ModActor_C"))
  (Variables|Default|SetModActor _returnvalue)
  (Utilities|FlowControl|Sequence
    (:then_0
      (bind _returnvalue_2 (Audio|SpawnSound2D "/Game/Mods/ChaosMod/Content/Audio/Wobble.Wobble" 1.0 1.0 0.0 0))
      (EventDispatchers|AssignOnAudioFinished _returnvalue_2 (delegate Custom|OnAudioFinished)))
    (:then_1
      (bind _returnvalue_3 (Rendering|Material|CreateDynamicMaterialInstance "/Game/Mods/ChaosMod/Content/Materials/PP_Wobble.PP_Wobble" "None" "None" :!class /Script/Engine.KismetMaterialLibrary))
      (Utilities|Array|AppendArray (.array (Utilities|Struct|BreakPostProcessSettings (Variables|/Script/Engine.PostProcessComponent|GetSettings (Variables|/Game/Mods/ChaosMod/ModActor.ModActor_C|GetPostProcess (Variables|Default|GetModActor))))) (Utilities|Array|MakeArray (Utilities|Struct|MakeWeightedBlendable 1.0 _returnvalue_3))))
    (:then_2
      (Utilities|FlowControl|Delay 2.25)
      (Variables|Default|Setx 0.0)
      (Utilities|FlowControl|Delay 2.25)
      (Variables|Default|Setx 0.0)
      (Utilities|FlowControl|Delay 2.25)
      (Variables|Default|Setx 0.0))))

(fn ConstructionScript)