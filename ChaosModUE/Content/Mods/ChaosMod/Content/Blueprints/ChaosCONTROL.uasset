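; ChaosMod remote-control actor that decodes commands hidden in a downloaded image, though its download chain is unwired and never runs.
; ReadData draws the texture to a render target and reads RGBA values as a command ID plus ASCII-mapped, delimited arguments.
; A switch dispatches overlay messages or media, ModActor events and next-event text, arbitrary console commands, URL launches, KillGregory and inventory changes.
; BeginPlay only caches the ModActor.
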(event EventBeginPlay
  (bind _returnvalue (Actor|GetActorOfClass "/Game/Mods/ChaosMod/ModActor.ModActor_C"))
  (Variables|Default|SetModActor _returnvalue))

(fn ConstructionScript)

(fn ReadData
  (params (Texture :type Texture%20Object%20Reference))
  (bind _loc_values (LocalVariables|GetLoc_Values))
  (bind _loc_values_2 (LocalVariables|GetLoc_Values))
  (bind _loc_data (LocalVariables|GetLoc_Data))
  (bind _loc_index (LocalVariables|GetLoc_Index))
  (bind _output (Utilities|Array|Get(acopy) _loc_data _loc_index))
  (bind _returnvalue (Rendering|CreateRenderTarget2D 999 999 "RTF_RGBA16f"))
  (bind _canvas (Rendering|BeginDrawCanvastoRenderTarget _returnvalue))
  (Canvas|DrawTexture :self _canvas :RenderTexture Texture :ScreenSize "(X=180.000000,Y=1.000000)" :CoordinateSize "(X=1.000000,Y=1.000000)" :BlendMode "BLEND_Opaque" :PivotPoint "(X=0.500000,Y=0.500000)")
  (bind _index (Utilities|FlowControl|ForLoopwithBreak 0 180 :!label _label)
    (:LoopBody
      (bind _returnvalue_2 (Class|KismetRenderingLibrary|ReadRenderTargetPixel _returnvalue _index))
      (Utilities|Array|Add _loc_values (Math|Conversions|ToInteger(Byte) (.r (Math|Conversions|ToColor(LinearColor) (Math|Conversions|ToLinearColor(Color) _returnvalue_2)))))
      (Utilities|Array|Add _loc_values (Math|Conversions|ToInteger(Byte) (.g (Math|Conversions|ToColor(LinearColor) (Math|Conversions|ToLinearColor(Color) _returnvalue_2)))))
      (Utilities|Array|Add _loc_values (Math|Conversions|ToInteger(Byte) (.b (Math|Conversions|ToColor(LinearColor) (Math|Conversions|ToLinearColor(Color) _returnvalue_2)))))
      (Utilities|Array|Add _loc_values (Math|Conversions|ToInteger(Byte) (.a (Math|Conversions|ToColor(LinearColor) (Math|Conversions|ToLinearColor(Color) _returnvalue_2)))))
      (if (Math|Boolean|ORBoolean (== (Math|Conversions|ToInteger(Byte) (.r (Math|Conversions|ToColor(LinearColor) (Math|Conversions|ToLinearColor(Color) _returnvalue_2)))) 31) (== (Math|Conversions|ToInteger(Byte) (.g (Math|Conversions|ToColor(LinearColor) (Math|Conversions|ToLinearColor(Color) _returnvalue_2)))) 31) (== (Math|Conversions|ToInteger(Byte) (.b (Math|Conversions|ToColor(LinearColor) (Math|Conversions|ToLinearColor(Color) _returnvalue_2)))) 31) (== (Math|Conversions|ToInteger(Byte) (.a (Math|Conversions|ToColor(LinearColor) (Math|Conversions|ToLinearColor(Color) _returnvalue_2)))) 31))
        (goto _label Break)))
    (:Completed
      (LocalVariables|SetLoc_Command (Utilities|Array|Get(acopy) _loc_values_2))
      (Utilities|Array|RemoveIndex _loc_values_2)
      (for _array_element _loc_values_2
        (if (== _array_element 30)
          (Math|Integer|IncrementInt _loc_index)
          (else
            (|SetBy-RefVar _output (Utilities|String|Append _output (Utilities|Array|Get(acopy) (LocalVariables|GetLoc_ASCII) _array_element))))))
      (return (LocalVariables|GetLoc_Command) (LocalVariables|GetLoc_Data)))))