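; NoTextures is a ChaosMod event that strips the look of the world by replacing mesh materials with WorldGridMaterial.
; Tick drives a 0.75-second DelayAbsolute, then rescans all actors only when the actor count differs from the cached Length.
; Each actor without a "Notex" tag receives the tag and has every material slot on its mesh components overwritten.
; The file contains no logic to restore the original materials.
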(event EventTick
  (params (DeltaSeconds :type Float%20%28single-precision%29))
  (Utilities|Delay(absolute) 0.75
    (:Completed
      (bind _outactors (Actor|GetAllActorsOfClass "/Script/Engine.Actor"))
      (if (!= (Utilities|Array|Length _outactors) (Variables|Default|GetLength))
        (Variables|Default|SetLength (Utilities|Array|Length _outactors))
        (for _array_element _outactors
          (if (not (Utilities|Array|ContainsItem (Variables|/Script/Engine.Actor|GetTags _array_element) "Notex"))
            (Utilities|Array|Add (Variables|/Script/Engine.Actor|GetTags _array_element) "Notex")
            (for _array_element_2 (Actor|GetComponentsByClass _array_element "/Script/Engine.MeshComponent")
              (for (_ _array_index) (Rendering|Material|GetMaterials _array_element_2)
                (Rendering|Material|SetMaterial _array_element_2 _array_index "/Engine/EngineMaterials/WorldGridMaterial.WorldGridMaterial")))))))))

(fn ConstructionScript)