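; Gun is a ChaosMod event actor that gives the player a hitscan gun for deleting enemy characters.
; It adds a reticle widget on spawn and follows just ahead of the player each tick, facing the control rotation.
; Left click plays a Bonk sound and line-traces along the view, ignoring Gregory and both Freddy actors.
; A cast chain destroys hit animatronics, bosses, Vanny, Vanessa or security StaffBots.
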(event EventBeginPlay
  (Collision|SetActorEnableCollision false)
  (bind _returnvalue (UserInterface|CreateWidget "/Game/Mods/ChaosMod/Content/Widgets/Reticle.Reticle_C"))
  (UserInterface|Viewport|AddtoViewport _returnvalue 9999))

(event EventTick
  (params (DeltaSeconds :type Float%20%28single-precision%29))
  (bind _returnvalue (Game|GetPlayerCharacter 0))
  (Transformation|SetActorLocationAndRotation (+ (* (Transformation|GetActorForwardVector _returnvalue) 4e+01) (Transformation|GetActorLocation _returnvalue)) (Pawn|GetControlRotation _returnvalue :!class /Script/Engine.Pawn)))

(event Input|MouseEvents|LeftMouseButton
  (params (Key :type Key%20Structure :default "None"))
  (bind _returnvalue (Game|GetPlayerCharacter 0))
  (bind _returnvalue_2 (Transformation|GetActorLocation _returnvalue))
  (bind _returnvalue_3 (+ _returnvalue_2 "0, 0,50.000000"))
  (:Pressed
    (Audio|PlaySound2D "/Game/Mods/ChaosMod/Content/Audio/Bonk.Bonk" 1.0 1.0 0.0 0 0)
    (bind _returnvalue_4 (Actor|GetActorOfClass "/Game/Blueprints/Player/Freddy.Freddy_C"))
    (bind _returnvalue_5 (Actor|GetActorOfClass "/Game/Blueprints/Player/Burntrap_Freddy.Burntrap_Freddy_C"))
    (bind _returnvalue_6 (Actor|GetActorOfClass "/Game/Blueprints/Player/Gregory.Gregory_C"))
    (bind _outhit (Collision|LineTraceByChannel _returnvalue_3 (+ _returnvalue_3 (* (Math|Vector|GetForwardVector (Pawn|GetControlRotation _returnvalue :!class /Script/Engine.Pawn)) 5e+04)) "TraceTypeQuery1" true (Utilities|Array|MakeArray _returnvalue_6 _returnvalue_4 _returnvalue_5) "None" true "(R=1.000000,G=0.000000,B=0.000000,A=1.000000)" "(R=0.000000,G=1.000000,B=0.000000,A=1.000000)" 1.0))
    (Utilities|Casting|CastToMonty (.hitactor _outhit)
      (:then
        _)
      (:CastFailed
        (Utilities|Casting|CastToshatteredMonty (.hitactor _outhit)
          (:then
            _)
          (:CastFailed
            (Utilities|Casting|CastToMontyShowtimeMission (.hitactor _outhit)
              (:then
                _)
              (:CastFailed
                (Utilities|Casting|CastToChica (.hitactor _outhit)
                  (:then
                    _)
                  (:CastFailed
                    (Utilities|Casting|CastToshatteredChica (.hitactor _outhit)
                      (:then
                        _)
                      (:CastFailed
                        (Utilities|Casting|CastToRoxy (.hitactor _outhit)
                          (:then
                            _)
                          (:CastFailed
                            (Utilities|Casting|CastToshatteredRoxy (.hitactor _outhit)
                              (:then
                                _)
                              (:CastFailed
                                (Utilities|Casting|CastToVanny (.hitactor _outhit)
                                  (:then
                                    _)
                                  (:CastFailed
                                    (Utilities|Casting|CastToVanessa (.hitactor _outhit)
                                      (:then
                                        _)
                                      (:CastFailed
                                        (Utilities|Casting|CastToBurnTrap (.hitactor _outhit)
                                          (:then
                                            _)
                                          (:CastFailed
                                            (Utilities|Casting|CastToTangleBlob (.hitactor _outhit)
                                              (:then
                                                _)
                                              (:CastFailed
                                                (Utilities|Casting|CastToDJMusicMan (.hitactor _outhit)
                                                  (:then
                                                    _)
                                                  (:CastFailed
                                                    (Utilities|Casting|CastToStaffBotSecurityPatrol (.hitactor _outhit))))))))))))))))))))))))))
    (Actor|DestroyActor (.hitactor _outhit))))

(fn ConstructionScript)