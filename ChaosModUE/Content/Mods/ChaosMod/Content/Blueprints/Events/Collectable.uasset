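; A Chaos Mod event pickup that completes a task in the Tattletail widget when Gregory touches it.
; On BeginPlay it traces straight down on the Visibility channel and snaps itself to the hit point.
; When its sphere overlaps Gregory, it sets Task3 on each top-level Tattletail widget and destroys itself inside that loop, so it remains if no such widget exists.
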(event OnComponentBeginOverlap(Sphere)
  (params (OverlappedComponent :type Primitive%20Component%20Object%20Reference) (OtherActor :type Actor%20Object%20Reference) (OtherComp :type Primitive%20Component%20Object%20Reference) (OtherBodyIndex :type Integer) (bFromSweep :type Boolean) (SweepResult :type Hit%20Result%20Structure%20%28by%20ref%29))
  (Utilities|Casting|CastToGregory OtherActor)
  (bind _foundwidgets (Widget|GetAllWidgetsOfClass "/Game/Mods/ChaosMod/Content/Blueprints/Widgets/Events/Tattletail.Tattletail_C" true))
  (for _array_element _foundwidgets
    (Variables|/Game/Mods/ChaosMod/Content/Blueprints/Widgets/Events/Tattletail.Tattletail_C|SetTask3 _array_element true)
    (Actor|DestroyActor)))

(event EventBeginPlay
  (bind _returnvalue (Transformation|GetActorLocation))
  (bind (_outhit _returnvalue_2) (Collision|LineTraceByChannel _returnvalue (- _returnvalue "0, 0,50000.000000") "TraceTypeQuery1" false 0 "None"))
  (if _returnvalue_2
    (Transformation|SetActorLocation (.ImpactPoint (Collision|BreakHitResult _outhit)) false false)))

(fn ConstructionScript)