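; Actor component for ChaosMod events that replaces its owner's normal gravity with a custom directional force while switched on.
; BeginPlay caches the owner's gravity-enabled, physics-simulating primitives and, for Characters, the original movement gravity scale.
; SetCustomGravity toggles built-in gravity on both and stores the direction.
; Tick pushes non-Character primitives with mass-dependent force, or Characters via CharacterMovement in Falling mode, skipping the grounded local player.
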(event Custom|SetCustomGravity
  (params (On :type Boolean) (Direction :type Vector))
  (bind _ischaracter (Variables|Default|GetIsCharacter))
  (bind _components (Variables|Default|GetComponents))
  (bind _output_get (Variables|Default|SetCustomGravityEnabled? On))
  (if _output_get
    (for _array_element _components
      (Physics|SetEnableGravity _array_element false))
    (Variables|Default|SetCustom%20Gravity%20Direction Direction)
    (if _ischaracter
      (Variables|/Script/Engine.CharacterMovementComponent|SetGravityScale (Variables|/Script/Engine.Character|GetCharacterMovement (Variables|Default|GetAs%20Character)) 0.0))
    (else
      (for _array_element_2 _components
        (Physics|SetEnableGravity _array_element_2 true))
      (if _ischaracter
        (bind _ascharacter (Utilities|Casting|CastToCharacter (Components|GetOwner)))
        (Variables|/Script/Engine.CharacterMovementComponent|SetGravityScale (Variables|/Script/Engine.Character|GetCharacterMovement _ascharacter) (Variables|Default|GetGravity%20Scale))))))

(event EventBeginPlay
  (bind _returnvalue (Components|GetOwner))
  (Utilities|Array|Clear (Variables|Default|GetComponents))
  (for _array_element (Actor|GetComponentsByClass _returnvalue "/Script/Engine.PrimitiveComponent")
    (if (and (Physics|IsSimulatingPhysics _array_element "None") (Class|PrimitiveComponent|IsGravityEnabled _array_element))
      (Utilities|Array|Add (Variables|Default|GetComponents) _array_element)))
  (bind _ascharacter (Utilities|Casting|CastToCharacter _returnvalue))
  (Variables|Default|SetGravity%20Scale (Variables|/Script/Engine.CharacterMovementComponent|GetGravityScale (Variables|/Script/Engine.Character|GetCharacterMovement _ascharacter)))
  (Variables|Default|SetIsCharacter true)
  (Variables|Default|SetAs%20Character _ascharacter))

(event EventTick
  (params (DeltaSeconds :type Float%20%28single-precision%29))
  (bind _as_character (Variables|Default|GetAs%20Character))
  (bind _custom_gravity_direction (Variables|Default|GetCustom%20Gravity%20Direction))
  (bind _charactermovement (Variables|/Script/Engine.Character|GetCharacterMovement _as_character))
  (if (Variables|Default|GetCustomGravityEnabled?)
    (if (Variables|Default|GetIsCharacter)
      (if (not (and (AI|Components|NavMovement|IsMovingonGround _charactermovement) (== _as_character (Game|GetPlayerCharacter 0))))
        (Physics|AddForce _charactermovement _custom_gravity_direction)
        (Pawn|Components|CharacterMovement|SetMovementMode _charactermovement "MOVE_Falling" 0))
      (else
        (for _array_element (Variables|Default|GetComponents)
          (Physics|AddForce _array_element _custom_gravity_direction "None" false))))))