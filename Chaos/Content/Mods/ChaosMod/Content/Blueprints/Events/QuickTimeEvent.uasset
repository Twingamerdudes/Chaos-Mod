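; Chaos Mod event actor that runs a slow-motion quick time event.
; On BeginPlay a timeline eases global time dilation down, then creates the QuickTime widget with itself as owner.
; End eases time back to normal speed with a second timeline, while Fail kills Gregory.
; A node that would delete the current save game is left unconnected and never runs.
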(event Custom|End
  (bind _newtrack_0 (Timeline|Timeline_0 PlayFromStart)
    (:Update
      (Utilities|Time|SetGlobalTimeDilation (Math|Float|Lerp 0.2 1.0 _newtrack_0)))))

(event Custom|Fail
  (CallFunction|KillGregory))

(event EventBeginPlay
  (bind _newtrack_0 (Timeline|Ease PlayFromStart)
    (:Update
      (Utilities|Time|SetGlobalTimeDilation (Math|Float|Lerp 1.0 0.2 _newtrack_0)))
    (:Finished
      (bind _returnvalue (UserInterface|CreateWidget "/Game/Mods/ChaosMod/Content/Widgets/Events/QuickTime.QuickTime_C" 0 self))
      (UserInterface|Viewport|AddtoViewport _returnvalue 0))))

(fn ConstructionScript)