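; Chaos mod event actor that makes the player's view lag by showing camera frames a few ticks late.
; BeginPlay hides the pawn, snaps a scene capture to the player camera and adds a high Z-order Delay widget.
; Tick cycles the capture target through a render-target ring buffer, displaying the oldest frame via a dynamic UI material.
; Only five of the ten listed render targets are used.
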(event EventBeginPlay
  (bind _returnvalue (Game|Player|GetPlayerPawn 0))
  (bind _returnvalue_2 (Actor|GetComponentbyClass _returnvalue "/Script/Engine.CameraComponent"))
  (Rendering|SetVisibility _returnvalue_2 false false)
  (Rendering|SetActorHiddenInGame _returnvalue true)
  (Transformation|AttachComponentToComponent (Variables|Default|GetSceneCaptureComponent2D) _returnvalue_2 "None" "SnapToTarget" "SnapToTarget" "SnapToTarget" true)
  (bind _returnvalue_3 (UserInterface|CreateWidget "/Game/Mods/ChaosMod/Content/Blueprints/Widgets/Events/Delay.Delay_C"))
  (bind _output_get (Variables|Default|SetDisplayWidget _returnvalue_3))
  (UserInterface|Viewport|AddtoViewport _output_get 1000)
  (bind _returnvalue_4 (Rendering|Material|CreateDynamicMaterialInstance "/Game/Mods/ChaosMod/Content/Materials/UI_Delay.UI_Delay" "None" "None" :!class /Script/Engine.KismetMaterialLibrary))
  (Variables|Default|SetDisplayMaterial _returnvalue_4)
  (Variables|Default|SetRT_Array (Utilities|Array|MakeArray "/Game/Mods/ChaosMod/Content/Textures/RenderTargets/RT_Frame_0.RT_Frame_0" "/Game/Mods/ChaosMod/Content/Textures/RenderTargets/RT_Frame_1.RT_Frame_1" "/Game/Mods/ChaosMod/Content/Textures/RenderTargets/RT_Frame_2.RT_Frame_2" "/Game/Mods/ChaosMod/Content/Textures/RenderTargets/RT_Frame_3.RT_Frame_3" "/Game/Mods/ChaosMod/Content/Textures/RenderTargets/RT_Frame_4.RT_Frame_4" "/Game/Mods/ChaosMod/Content/Textures/RenderTargets/RT_Frame_5.RT_Frame_5" "/Game/Mods/ChaosMod/Content/Textures/RenderTargets/RT_Frame_6.RT_Frame_6" "/Game/Mods/ChaosMod/Content/Textures/RenderTargets/RT_Frame_7.RT_Frame_7" "/Game/Mods/ChaosMod/Content/Textures/RenderTargets/RT_Frame_8.RT_Frame_8" "/Game/Mods/ChaosMod/Content/Textures/RenderTargets/RT_Frame_9.RT_Frame_9")))

(event EventTick
  (params (DeltaSeconds :type Float%20%28single-precision%29))
  (bind _rt_array (Variables|Default|GetRT_Array))
  (bind _output_get (Variables|Default|SetFrameIndex (Math|Integer|%(Integer) (+ (Variables|Default|GetFrameIndex) 1) 5)))
  (Variables|/Script/Engine.SceneCaptureComponent2D|SetTextureTarget (Variables|Default|GetSceneCaptureComponent2D) (Utilities|Array|Get(acopy) _rt_array _output_get))
  (Rendering|Material|SetTextureParameterValue (Variables|Default|GetDisplayMaterial) "DisplayTexture" (Utilities|Array|Get(acopy) _rt_array (Math|Integer|%(Integer) (+ _output_get 1) 5)))
  (Class|Image|SetBrushfromMaterial (Variables|/Game/Mods/ChaosMod/Content/Blueprints/Widgets/Events/Delay.Delay_C|GetScreenDisplay (Variables|Default|GetDisplayWidget)) (Variables|Default|GetDisplayMaterial)))

(fn ConstructionScript)