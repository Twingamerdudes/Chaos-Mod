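; Chaos mod item handler that applies gameplay perks according to numbered flags in an Items map, auto-granting the recharge perk on the DLC world map.
; Tick refreshes Fazcam and Fazerblaster references on a short delay and polls the flags.
; Active perks halve time dilation on registered AI, security staff bots and map bots, keep both weapons recharged, or give Gregory one 30-second jumpscare immunity.
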(event EventTick
  (params (DeltaSeconds :type Float%20%28single-precision%29))
  (bind _items (Variables|Default|GetItems))
  (Utilities|FlowControl|Sequence
    (:then_0
      (Utilities|FlowControl|Delay 0.2)
      (bind _returnvalue (Actor|GetActorOfClass "/Game/Blueprints/Objects/Equippables/EQ_Flashbeacon.EQ_Flashbeacon_C"))
      (Variables|Default|SetFazcam _returnvalue)
      (bind _returnvalue_2 (Actor|GetActorOfClass "/Game/Blueprints/Objects/Equippables/EQ_LaserGun.EQ_LaserGun_C"))
      (Variables|Default|SetFazerblaster _returnvalue_2))
    (:then_1
      (if (.Value (Utilities|Map|Find _items 2))
        (Utilities|FlowControl|Delay 0.2)
        (for _array_element (Class|AIManagementSystem|GetAllRegisteredAI (Subsystems|GetAIManagementSystem))
          (Variables|/Script/Engine.Actor|SetCustomTimeDilation _array_element 0.5))
        (bind _outactors (Actor|GetAllActorsOfClass "/Game/Blueprints/AI/StaffBot/Security/Patrol/StaffBotSecurityPatrol.StaffBotSecurityPatrol_C"))
        (for _array_element_2 _outactors
          (Variables|/Script/Engine.Actor|SetCustomTimeDilation _array_element_2 0.5))
        (bind _outactors_2 (Actor|GetAllActorsOfClass "/Game/Blueprints/AI/StaffBot/MapBot/MapBot.MapBot_C"))
        (for _array_element_3 _outactors_2
          (Variables|/Script/Engine.Actor|SetCustomTimeDilation _array_element_3 0.5))))
    (:then_2
      (if (.Value (Utilities|Map|Find _items 3))
        (Utilities|FlowControl|Sequence
          (:then_0
            (if (<= (Variables|/Game/Blueprints/Objects/Equippables/EQ_LaserGun.EQ_LaserGun_C|GetShotsLeft (Variables|Default|GetFazerblaster)) 5)
              (Default|Recharge (Variables|Default|GetFazerblaster))))
          (:then_1
            (if (not (Variables|/Game/Blueprints/Objects/Equippables/EQ_Flashbeacon.EQ_Flashbeacon_C|GetCanUse? (Variables|Default|GetFazcam)))
              (Utilities|FlowControl|DoOnce false :!label _label
                (:Completed
                  (Default|Recharging (Variables|Default|GetFazcam))
                  (Utilities|FlowControl|Delay 1.2)
                  (goto _label Reset))))))))
    (:then_3
      (if (.Value (Utilities|Map|Find _items 7))
        (Utilities|FlowControl|DoOnce false
          (:Completed
            (bind _asgregory (Utilities|Casting|CastToGregory (Game|GetPlayerCharacter 0)))
            (Variables|/Game/Blueprints/Player/Gregory.Gregory_C|SetCanBeJumpScared _asgregory false)
            (Utilities|FlowControl|Delay 3e+01)
            (Variables|/Game/Blueprints/Player/Gregory.Gregory_C|SetCanBeJumpScared _asgregory true)))))))

(event EventBeginPlay
  (Utilities|CurrentLevel "MAP_World_DLC"
    (:true
      (Utilities|Map|Add (Variables|Default|GetItems) 3 true)
      (bind _returnvalue (Actor|GetActorOfClass "/Game/Blueprints/Objects/Equippables/EQ_Flashbeacon.EQ_Flashbeacon_C"))
      (Variables|Default|SetFazcam _returnvalue)
      (bind _returnvalue_2 (Actor|GetActorOfClass "/Game/Blueprints/Objects/Equippables/EQ_LaserGun.EQ_LaserGun_C"))
      (Variables|Default|SetFazerblaster _returnvalue_2))))

(fn ConstructionScript)