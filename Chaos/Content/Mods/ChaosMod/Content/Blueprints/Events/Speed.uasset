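; Chaos Mod event actor that makes Gregory's movement extremely fast for a timed period.
; On BeginPlay it finds Gregory and caches greatly multiplied copies of his walk speed, crouched speed and acceleration.
; Tick reapplies those values to his CharacterMovement while a flag is set.
; After a delay it clears the flag and destroys itself, without restoring the original values.
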(event EventBeginPlay
  (bind _returnvalue (Actor|GetActorOfClass "/Game/Blueprints/Player/Gregory.Gregory_C"))
  (Variables|Default|SetMax%20Speed (* 50 (Variables|/Script/Engine.CharacterMovementComponent|GetMaxWalkSpeed (Variables|/Script/Engine.Character|GetCharacterMovement _returnvalue))))
  (Variables|Default|SetMax%20Acceleration (* 50 (Variables|/Script/Engine.CharacterMovementComponent|GetMaxAcceleration (Variables|/Script/Engine.Character|GetCharacterMovement _returnvalue))))
  (Variables|Default|SetMax%20Speed%20Crouched (* 50 (Variables|/Script/Engine.CharacterMovementComponent|GetMaxWalkSpeedCrouched (Variables|/Script/Engine.Character|GetCharacterMovement _returnvalue))))
  (Variables|Default|SetSpeed? true)
  (Utilities|FlowControl|Delay 3e+01)
  (Variables|Default|SetSpeed? false)
  (Actor|DestroyActor))

(event EventTick
  (params (DeltaSeconds :type Float%20%28single-precision%29))
  (if (Variables|Default|GetSpeed?)
    (Variables|/Script/Engine.CharacterMovementComponent|SetMaxWalkSpeed (Variables|/Script/Engine.Character|GetCharacterMovement (stale EventBeginPlay _returnvalue)) (Variables|Default|GetMax%20Speed))
    (Variables|/Script/Engine.CharacterMovementComponent|SetMaxWalkSpeedCrouched (Variables|/Script/Engine.Character|GetCharacterMovement (stale EventBeginPlay _returnvalue)) (Variables|Default|GetMax%20Speed%20Crouched))
    (Variables|/Script/Engine.CharacterMovementComponent|SetMaxAcceleration (Variables|/Script/Engine.Character|GetCharacterMovement (stale EventBeginPlay _returnvalue)) (Variables|Default|GetMax%20Acceleration))))

(fn ConstructionScript)