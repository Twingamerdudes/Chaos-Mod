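; FazCoin is a collectible coin pickup actor for ChaosMod events.
; On BeginPlay it traces straight down to snap itself onto the ground, then destroys itself after a timed lifetime.
; When Gregory, Freddy or Burntrap Freddy overlaps its sphere, it increments the Coins counter on the ModActor and destroys itself.
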(event OnComponentBeginOverlap(Sphere)
  (params (OverlappedComponent :type Primitive%20Component%20Object%20Reference) (OtherActor :type Actor%20Object%20Reference) (OtherComp :type Primitive%20Component%20Object%20Reference) (OtherBodyIndex :type Integer) (bFromSweep :type Boolean) (SweepResult :type Hit%20Result%20Structure%20%28by%20ref%29))
  (Utilities|Casting|CastToGregory OtherActor
    (:then
      _)
    (:CastFailed
      (Utilities|Casting|CastToFreddy OtherActor
        (:then
          _)
        (:CastFailed
          (Utilities|Casting|CastToBurntrap_Freddy OtherActor)))))
  (bind _returnvalue (Actor|GetActorOfClass "/Game/Mods/ChaosMod/ModActor.ModActor_C"))
  (Math|Integer|IncrementInt (Variables|/Game/Mods/ChaosMod/ModActor.ModActor_C|GetCoins _returnvalue)
    (:%20%20
      (Actor|DestroyActor))))

(event EventBeginPlay
  (bind _returnvalue (Transformation|GetActorLocation))
  (Utilities|FlowControl|Sequence
    (:then_0
      (bind (_outhit _returnvalue_2) (Collision|LineTraceByChannel _returnvalue (- _returnvalue "0, 0,50000.000000") "TraceTypeQuery1" false 0 "None"))
      (if _returnvalue_2
        (Transformation|SetActorLocation (.ImpactPoint (Collision|BreakHitResult _outhit)) false false)))
    (:then_1
      (Utilities|FlowControl|Delay 1e+01)
      (Actor|DestroyActor))))

(fn ConstructionScript)